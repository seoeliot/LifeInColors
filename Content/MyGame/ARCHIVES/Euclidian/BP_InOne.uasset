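; Non-Euclidean-style actor that changes a door and wall as the player character passes through its trigger boxes.
; Overlapping Box destroys the wall (Mur) and that trigger.
; BoxIn and BoxOut track crossing order with two flags: reaching BoxOut without a pending BoxIn arms the change, and the next BoxIn overlap swaps Porte to NewPorte and removes both triggers.
; The construction script sets the door's initial mesh to LastPort.
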(event `self.Box.OnComponentBeginOverlap`
  (params (OverlappedComponent :type "PrimitiveComponent Object Reference") (OtherActor :type "Actor Object Reference") (OtherComp :type "PrimitiveComponent Object Reference") (OtherBodyIndex :type Integer) (bFromSweep :type Boolean) (SweepResult :type "HitResult Structure (by ref)"))
  (if (== OtherActor (`GameplayStatics.GetPlayerCharacter` 0))
    (`ActorComponent.K2_DestroyComponent` (`self.Mur`))
    (`ActorComponent.K2_DestroyComponent` (`self.Box`))))

(event `self.BoxIn.OnComponentBeginOverlap`
  (params (OverlappedComponent :type "PrimitiveComponent Object Reference") (OtherActor :type "Actor Object Reference") (OtherComp :type "PrimitiveComponent Object Reference") (OtherBodyIndex :type Integer) (bFromSweep :type Boolean) (SweepResult :type "HitResult Structure (by ref)"))
  (if (== OtherActor (`GameplayStatics.GetPlayerCharacter` 0))
    (if (`self.FirstOut`)
      (`StaticMeshComponent.SetStaticMesh` (`self.Porte`) (`self.NewPorte`))
      (`ActorComponent.K2_DestroyComponent` (`self.BoxOut`))
      (`ActorComponent.K2_DestroyComponent` (`self.BoxIn`))
      (else
        (set `self.FirstIn` true)))))

(event `self.BoxOut.OnComponentBeginOverlap`
  (params (OverlappedComponent :type "PrimitiveComponent Object Reference") (OtherActor :type "Actor Object Reference") (OtherComp :type "PrimitiveComponent Object Reference") (OtherBodyIndex :type Integer) (bFromSweep :type Boolean) (SweepResult :type "HitResult Structure (by ref)"))
  (if (== OtherActor (`GameplayStatics.GetPlayerCharacter` 0))
    (if (`self.FirstIn`)
      (set `self.FirstIn` false)
      (else
        (set `self.FirstOut` true)))))

(fn `UserConstructionScript`
  (`StaticMeshComponent.SetStaticMesh` (`self.Porte`) (`self.LastPort`)))