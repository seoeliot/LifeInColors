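; BP_teleporteur is a teleporter actor that moves the first-person player when they overlap its Box component.
; On overlap it casts to BP_FirstPerson and teleports it without sweep to the Destination offset added to an actor location, then prints the sweep hit location as debug output.
; The construction script writes the Text variable to a TextRender label.
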(event `self.Box.OnComponentBeginOverlap`
  (params (OverlappedComponent :type "PrimitiveComponent Object Reference") (OtherActor :type "Actor Object Reference") (OtherComp :type "PrimitiveComponent Object Reference") (OtherBodyIndex :type Integer) (bFromSweep :type Boolean) (SweepResult :type "HitResult Structure (by ref)"))
  (bind _asbp_first_person (cast `/Game/MyGame/Joueur/Character/BP_FirstPerson` OtherActor))
  (bind _sweephitresult (`self.K2_SetActorLocation` _asbp_first_person (+ (`self.destination`) (`self.K2_GetActorLocation`)) false true))
  (`KismetSystemLibrary.PrintString` (`KismetStringLibrary.Conv_VectorToString` (`.Location` (`GameplayStatics.BreakHitResult` _sweephitresult)))))

(fn `UserConstructionScript`
  (`TextRenderComponent.K2_SetText` (`self.TextRender`) (`self.Text`)))