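; Portal clone actor for a static mesh, part of an archived portal system.
; Each Tick it adds the mesh's linear and angular velocities to running stored totals, then zeroes both on the physics body.
; This keeps cancelling the clone's own physics motion while capturing it in StoredVel and StoredAngularVel; nothing in this Blueprint consumes or resets those totals.
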(event `self.ReceiveTick`
  (params (DeltaSeconds :type "Float (single-precision)"))
  (bind _staticmesh (`self.StaticMesh`))
  (set `self.StoredVel` (+ (`SceneComponent.GetComponentVelocity` _staticmesh) (`self.StoredVel`)))
  (`PrimitiveComponent.SetPhysicsLinearVelocity` _staticmesh (0.0 0.0 0.0) false "None")
  (set `self.StoredAngularVel` (+ (`PrimitiveComponent.GetPhysicsAngularVelocityInRadians` _staticmesh "None") (`self.StoredAngularVel`)))
  (`PrimitiveComponent.SetPhysicsAngularVelocityInRadians` _staticmesh (0.0 0.0 0.0) false "None"))

(fn `UserConstructionScript`)