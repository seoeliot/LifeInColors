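; Helper actor for the portal system that disables collision between a moving component and the blocking walls behind a portal and its target portal.
; On BeginPlay, physics-simulating primitives are bound to each wall through two physics constraints, apparently used only to switch off collision between the pair.
; Capsule components instead set IgnoreActorWhenMoving on each wall's owning actor.
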(event `self.ReceiveBeginPlay`
  (bind _portal (`self.Portal`))
  (bind _portal_2 (`self.Portal`))
  (bind _moveableactor (`self.MoveableActor`))
  (bind _blockingwall (`/Game/MyGame/ARCHIVES/Portal/Portal_NouvelleVersion/Blueprints/PortalBP.BlockingWall` _portal))
  (bind _blockingwall_2 (`/Game/MyGame/ARCHIVES/Portal/Portal_NouvelleVersion/Blueprints/PortalBP.BlockingWall` _portal_2))
  (bind _blockingwall_3 (`/Game/MyGame/ARCHIVES/Portal/Portal_NouvelleVersion/Blueprints/PortalBP.BlockingWall` (`/Game/MyGame/ARCHIVES/Portal/Portal_NouvelleVersion/Blueprints/PortalBP.TargetPortal` _portal_2)))
  (bind _blockingwall_4 (`/Game/MyGame/ARCHIVES/Portal/Portal_NouvelleVersion/Blueprints/PortalBP.BlockingWall` (`/Game/MyGame/ARCHIVES/Portal/Portal_NouvelleVersion/Blueprints/PortalBP.TargetPortal` _portal)))
  (`|ExecutionSequence`
    (:`then_0`
      (bind _asprimitive_component (cast `PrimitiveComponent` _moveableactor))
      ;[1 1 1] disable collision for primative
      (if (`SceneComponent.IsSimulatingPhysics` _asprimitive_component "None")
        (`|ExecutionSequence`
          (:`then_0`
            (`/Engine/EditorBlueprintResources/StandardMacros.IsValid` _blockingwall_4
              (:`Is Valid`
                (`PhysicsConstraintComponent.SetConstrainedComponents` (`self.PhysicsConstraint`) _asprimitive_component "None" _blockingwall_4 "None"))))
          (:`then_1`
            (`/Engine/EditorBlueprintResources/StandardMacros.IsValid` _blockingwall
              (:`Is Valid`
                (`PhysicsConstraintComponent.SetConstrainedComponents` (`self.PhysicsConstraint1`) _asprimitive_component "None" _blockingwall "None")))))))
    (:`then_1`
      ;[1 1 1] disable collision for capsule
      (bind _ascapsule_collision (cast `CapsuleComponent` _moveableactor))
      (`|ExecutionSequence`
        (:`then_0`
          (`/Engine/EditorBlueprintResources/StandardMacros.IsValid` _blockingwall_3
            (:`Is Valid`
              (`PrimitiveComponent.IgnoreActorWhenMoving` _ascapsule_collision (`ActorComponent.GetOwner` _blockingwall_3) true))))
        (:`then_1`
          (`/Engine/EditorBlueprintResources/StandardMacros.IsValid` _blockingwall_2
            (:`Is Valid`
              (`PrimitiveComponent.IgnoreActorWhenMoving` _ascapsule_collision (`ActorComponent.GetOwner` _blockingwall_2) true))))))))

(fn `UserConstructionScript`)