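; BP_Nemesis is an enemy character that pursues the player and destroys them on contact.
; On BeginPlay it sets its walk speed, saves its spawn transform in GM_InGame and starts chasing if the game mode's NemesisCanMoove flag is set.
; The chase is a self-restarting AIMoveTo loop that repeats on success or failure.
; Box overlap with the player destroys the player character and calls the game mode's VerifEtSpawnNemesis.
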(event `self.ReceiveBeginPlay`
  (set `CharacterMovementComponent.MaxWalkSpeed` (`self.SpeedNemesis`) (`self.CharacterMovement`))
  (bind _asgm_in_game (cast `/Game/MyGame/Data/GameInstance/GM_InGame` (`GameplayStatics.GetGameMode`)))
  (set `/Game/MyGame/Data/GameInstance/GM_InGame.SpawnTransformNemesis` (`self.GetTransform`) _asgm_in_game)
  (bind _asgm_in_game_2 (cast `/Game/MyGame/Data/GameInstance/GM_InGame` (`GameplayStatics.GetGameMode`)))
  (if (`/Game/MyGame/Data/GameInstance/GM_InGame.NemesisCanMoove` _asgm_in_game_2)
    (`self.GoToPlayer`)))

(event `GoToPlayer`
  (`|AIMoveTo` self (0.0 0.0 0.0) (`GameplayStatics.GetPlayerCharacter` 0)
    (:`OnSuccess`
      _)
    (:`OnFail`
      _))
  (`self.GoToPlayer`))

(event `self.Box.OnComponentBeginOverlap`
  (params (OverlappedComponent :type "PrimitiveComponent Object Reference") (OtherActor :type "Actor Object Reference") (OtherComp :type "PrimitiveComponent Object Reference") (OtherBodyIndex :type Integer) (bFromSweep :type Boolean) (SweepResult :type "HitResult Structure (by ref)"))
  (bind _returnvalue (`GameplayStatics.GetPlayerCharacter` 0))
  (if (== OtherActor _returnvalue)
    (`self.K2_DestroyActor` _returnvalue)
    (bind _asgm_in_game (cast `/Game/MyGame/Data/GameInstance/GM_InGame` (`GameplayStatics.GetGameMode`)))
    (`/Game/MyGame/Data/GameInstance/GM_InGame.VerifEtSpawnNemesis` _asgm_in_game)))

(fn `UserConstructionScript`)