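; BP_Compresseur is a compressor hazard that moves endlessly between two points offset from its placed location.
; A timeline lerps the mesh and reverses at each end, with per-instance time dilation and start time.
; At each end it plays audio if Bruit is enabled and BP_FirstPerson is inside the audio sphere.
; Box overlap with a TriggerMine-tagged actor sets Mort on GI_Main and destroys that actor.
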(event `self.ReceiveBeginPlay`
  (set `self.CustomTimeDilation` (`self.TimeDilation`))
  (set `self.BeginLoc` (+ (`self.K2_GetActorLocation`) (`self.BeginLoc`)))
  (set `self.EndLoc` (+ (`self.EndLoc`) (`self.K2_GetActorLocation`)))
  (`TimelineComponent.SetNewTime` (`self.Timeline_0`) (`self.Newtime`))
  (bind (_direction _newtrack_0) (`Timeline|Timeline_0` :!label _label)
    (:`Update`
      (`SceneComponent.K2_SetWorldLocation` (`self.Compresseur`) (`KismetMathLibrary.VLerp` (`self.BeginLoc`) (`self.EndLoc`) _newtrack_0) false false))
    (:`Finished`
      (if (`self.Bruit?`)
        (if (`self.SphereBruit`)
          (`ActorComponent.Activate` (`self.Audio`) true)))
      (switch `ETimelineDirection` _direction
        (:`Forward`
          (goto _label :!via `Reverse`))
        (:`Backward`
          (goto _label))))))

(event `self.BoxCollider.OnComponentBeginOverlap`
  (params (OverlappedComponent :type "PrimitiveComponent Object Reference") (OtherActor :type "Actor Object Reference") (OtherComp :type "PrimitiveComponent Object Reference") (OtherBodyIndex :type Integer) (bFromSweep :type Boolean) (SweepResult :type "HitResult Structure (by ref)"))
  (if (`self.ActorHasTag` OtherActor "TriggerMine")
    (bind _asgi_main (cast `/Game/MyGame/GameInstance/GI_Main` (`GameplayStatics.GetGameInstance`)))
    (set `/Game/MyGame/GameInstance/GI_Main.Mort?` true _asgi_main)
    (`self.K2_DestroyActor` OtherActor)))

(event `self.SphereAudio.OnComponentBeginOverlap`
  (params (OverlappedComponent :type "PrimitiveComponent Object Reference") (OtherActor :type "Actor Object Reference") (OtherComp :type "PrimitiveComponent Object Reference") (OtherBodyIndex :type Integer) (bFromSweep :type Boolean) (SweepResult :type "HitResult Structure (by ref)"))
  (cast `/Game/MyGame/Blueprint/BP_FirstPerson/BP_FirstPerson` OtherActor)
  (set `self.SphereBruit` true))

(event `self.SphereAudio.OnComponentEndOverlap`
  (params (OverlappedComponent :type "PrimitiveComponent Object Reference") (OtherActor :type "Actor Object Reference") (OtherComp :type "PrimitiveComponent Object Reference") (OtherBodyIndex :type Integer))
  (cast `/Game/MyGame/Blueprint/BP_FirstPerson/BP_FirstPerson` OtherActor)
  (set `self.SphereBruit` false))

(fn `UserConstructionScript`)