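; Progression manager that unlocks the room paths (CheminSalle1 to 4) according to the player's progress.
; BeginPlay and DeblocageEvent read ProgressionState from GI_Main, then open the current path and close later ones, leaving earlier paths untouched.
; ChangeAllCollisions recursively gathers each path's child actors and toggles collision and visibility on one primitive component per child.
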(event `DeblocageEvent`
  (bind _cheminsalle2 (`self.CheminSalle2`))
  (bind _cheminsalle1 (`self.CheminSalle1`))
  (bind _cheminsalle3 (`self.CheminSalle3`))
  (bind _cheminsalle4 (`self.CheminSalle4`))
  (bind _asgi_main (cast `/Game/MyGame/GameInstance/GI_Main` (`GameplayStatics.GetGameInstance`) :!label _label))
  (switch `/Game/MyGame/GameInstance/ProgressionState` (`/Game/MyGame/GameInstance/GI_Main.ProgressionState` _asgi_main)
    (:`NewEnumerator0`
      (`self.Change All Collisions` _cheminsalle1 false true)
      (`self.Change All Collisions` _cheminsalle2 false true)
      (`self.Change All Collisions` _cheminsalle3 false true)
      (`self.Change All Collisions` _cheminsalle4 false true))
    (:`NewEnumerator6`
      (`self.Change All Collisions` _cheminsalle1 true true)
      (`self.Change All Collisions` _cheminsalle2 false true)
      (`self.Change All Collisions` _cheminsalle3 false true)
      (`self.Change All Collisions` _cheminsalle4 false true))
    (:`NewEnumerator1`
      (`self.Change All Collisions` _cheminsalle2 true true)
      (`self.Change All Collisions` _cheminsalle3 false true)
      (`self.Change All Collisions` _cheminsalle4 false true))
    (:`NewEnumerator2`
      (`self.Change All Collisions` _cheminsalle3 true true)
      (`self.Change All Collisions` _cheminsalle4 false true))
    (:`NewEnumerator3`
      (`self.Change All Collisions` _cheminsalle4 true true))))

(event `self.ReceiveBeginPlay`
  (goto _label))

(fn `Change All Collisions`
  (params (Actor :type "Actor Object Reference") (ActivateCollision :type Boolean) (ChangeVisibility :type Boolean))
  (if (`KismetSystemLibrary.IsValid` Actor)
    ;[1 1 1] Looping through meshes
    (for _array_element (`self.GetAllChildActors` Actor true)
      (if (`KismetSystemLibrary.IsValid` _array_element)
        (for _array_element_2 (`|MakeArray` (`self.GetComponentByClass` _array_element "/Script/Engine.PrimitiveComponent") :!type "ActorComponent Object Reference")
          (bind _asprimitive_component (cast `PrimitiveComponent` _array_element_2))
          (if ActivateCollision
            (`PrimitiveComponent.SetCollisionEnabled` _asprimitive_component "QueryAndPhysics")
            (if ChangeVisibility
              (`SceneComponent.SetVisibility` _asprimitive_component true false))
            (else
              (`PrimitiveComponent.SetCollisionEnabled` _asprimitive_component "NoCollision")
              (if ChangeVisibility
                (`SceneComponent.SetVisibility` _asprimitive_component false false)))))))))

(fn `UserConstructionScript`)