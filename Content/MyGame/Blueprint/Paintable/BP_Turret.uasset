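; Paintable turret that detects tagged actors in a capsule and fires BP_TurretBullet, with behavior set by its color.
; Tick confirms line of sight with a sphere trace ignoring bullets, lerps the core toward the target, then fires after a color-dependent delay.
; Blue disables targeting and hides a beam, Green rotates the detection hitbox, and Red keeps firing even without a target.
; ChangeColor swaps the cannon material, forcing None when unpaintable.
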(event `self.ReceiveBeginPlay`
  (bind _rayontower (`self.RayonTower`))
  (bind _rayontower1 (`self.RayonTower1`))
  (`|ExecutionSequence`
    (:`then_0`
      (set `self.DefaultRotation` (`self.K2_GetActorRotation`))
      (add `self.OnChangeColor` (`|CreateDelegate` :!event `EventChangeColor`)))
    (:`then_1`
      (if (`self.UpdateLaser?`)
        (`ActorComponent.Activate` _rayontower false)
        (`ActorComponent.Deactivate` _rayontower1)
        (else
          (`ActorComponent.Activate` _rayontower1 false)
          (`ActorComponent.Deactivate` _rayontower))))))

(event `self.ReceiveTick`
  (params (DeltaSeconds :type "Float (single-precision)"))
  (bind _pointlight (`self.PointLight`))
  (if (`|EnumInequality` (`self.color`) "NewEnumerator0")
    (bind _targetableactors (`self.Get Targetable Actors`))
    (bind _output (`|GetArrayItem` _targetableactors))
    (`/Engine/EditorBlueprintResources/StandardMacros.IsValid` _output
      (:`Is Valid`
        (`SceneComponent.SetVisibility` _pointlight true false)
        (bind _outactors (`GameplayStatics.GetAllActorsOfClass` "/Game/MyGame/Blueprint/Paintable/BP_TurretBullet.BP_TurretBullet_C"))
        (bind _outhit (`KismetSystemLibrary.SphereTraceSingle` (`SceneComponent.K2_GetComponentLocation` (`self.canon`)) (`self.K2_GetActorLocation` _output) 10.0 "TraceTypeQuery1" true _outactors))
        (if (== (`.HitActor` (`GameplayStatics.BreakHitResult` _outhit)) _output)
          (`self.RotateToward` (`KismetMathLibrary.FindLookAtRotation` (`SceneComponent.K2_GetComponentLocation` (`self.turretCore`)) (`self.K2_GetActorLocation` _output)))
          (if (`self.HasTarget`)
            (`KismetSystemLibrary.Delay` (select `/Game/MyGame/Data/EnumColor` (`self.color`) :`NewEnumerator1` 0.05 :`NewEnumerator2` 0.05 :`NewEnumerator3` 0.1 :`NewEnumerator4` 0.1 :!type "Float (single-precision)"))
            (`self.FireBullet` _output)
            (goto _label :!via `Reset`)
            (else
              (`/Engine/EditorBlueprintResources/StandardMacros.DoOnce` false :!label _label
                (:`Completed`
                  (if (`|EnumEquality` (`self.color`) "NewEnumerator1")
                    (set `self.HasTarget` true)
                    (else
                      (`GameplayStatics.PlaySoundAtLocation` "/Game/MyGame/Sound/Unlock.Unlock" (`self.K2_GetActorLocation`) (struct) 1.0 1.0 0.0 null null null null)
                      (`KismetSystemLibrary.Delay` 0.3)
                      (set `self.HasTarget` true)
                      (`self.FireBullet` _output)))))))))
      (:`Is Not Valid`
        (`SceneComponent.SetVisibility` _pointlight false false)
        (`self.RotateToward` (`self.CurrentRotation`) true)
        (set `self.HasTarget` false)
        (if (`|EnumEquality` (`self.color`) "NewEnumerator1")
          (`KismetSystemLibrary.Delay` 0.05)
          (`self.FireBullet` null)
          (else
            (goto _label :!via `Reset`)))))))

(event `EventChangeColor`
  (`SceneComponent.SetVisibility` (`self.RayonTower`) true false)
  (`self.Reset`)
  (switch `/Game/MyGame/Data/EnumColor` (`self.color`)
    (:`NewEnumerator0`
      (`SceneComponent.SetVisibility` (`self.RayonTower`) false false))
    (:`NewEnumerator3`
      (`self.EventGreenRotation` (struct :`Yaw` 90.0)))))

(event `EventGreenRotation`
  (params (newRotation :type "Rotator Structure"))
  (bind (_returnvalue_x _returnvalue_y _returnvalue_z) (`KismetMathLibrary.BreakVector` (+ (`self.DefaultRotation`) (`KismetMathLibrary.MakeVector` newRotation_Roll newRotation_Pitch newRotation_Yaw))))
  (bind _output_get (set `self.CurrentRotation` (`KismetMathLibrary.MakeRotator` _returnvalue_x _returnvalue_y _returnvalue_z)))
  (`SceneComponent.K2_SetRelativeRotation` (`self.hitboxPivot`) _output_get false false))

(fn `changeColor`
  (params (newColor :type "/Game/MyGame/Data/EnumColor Enum" :default "NewEnumerator0"))
  (bind (_mat_none _mat_blue _mat_green _mat_yellow _mat_red) (break `/Game/MyGame/Data/StructColorText` (`self.colorTextures`)))
  (if (`self.Paintable`)
    (set `self.color` newColor)
    (`self.OnChangeColor`)
    (`PrimitiveComponent.SetMaterial` (`self.canon`) 0 (`|GetArrayItem` (select `/Game/MyGame/Data/EnumColor` (`self.color`) :`NewEnumerator0` _mat_blue :`NewEnumerator1` _mat_red :`NewEnumerator2` _mat_yellow :`NewEnumerator3` _mat_green :`NewEnumerator4` _mat_none)))
    (else
      (set `self.color` "NewEnumerator4")
      (`PrimitiveComponent.SetMaterial` (`self.canon`) 0 "/Game/UE5/StarterContent/Materials/M_Metal_Burnished_Steel.M_Metal_Burnished_Steel"))))

(fn `FireBullet`
  (params (target :type "Actor Object Reference"))
  (`|SpawnActorFromClass` "/Game/MyGame/Blueprint/Paintable/BP_TurretBullet.BP_TurretBullet_C" (`KismetMathLibrary.MakeTransform` (`SceneComponent.K2_GetComponentLocation` (`self.Sphere`)) (`KismetMathLibrary.Conv_VectorToRotator` (`SceneComponent.GetForwardVector` (`self.turretCore`))) (0.1 0.1 0.1)) "Undefined" "OverrideRootScale" null target (`self.color`) null)
  (if (`|EnumInequality` (`self.color`) "NewEnumerator1")
    (`GameplayStatics.PlaySoundAtLocation` "/Game/MyGame/Sound/TourellePiouPiou.TourellePiouPiou" (`SceneComponent.K2_GetComponentLocation` (`self.Cone`)) (struct) 1.0 1.0 0.0 null null null null)))

(fn `Get Targetable Actors`
  (returns (targetableActors :type "Array of Actor Object Reference"))
  (locals (NewLocalVar_0 :type "Array of Actor Object Reference") (actors :type "Array of Actor Object Reference"))
  (bind _output_get (set `local.NewLocalVar_0` (`PrimitiveComponent.GetOverlappingActors` (`self.Capsule`) null)))
  (for _array_element _output_get
    (if (`self.ActorHasTag` _array_element (`self.targetTag`))
      (`KismetArrayLibrary.Array_Add` (`local.actors`) _array_element)))
  (return (`local.actors`)))

(fn `Reset`
  (set `self.CurrentRotation` (struct))
  (`self.EventGreenRotation` (struct)))

(fn `RotateToward`
  (params (B :type "Rotator Structure") (isRelative :type Boolean))
  (bind _turretcore (`self.turretCore`))
  (bind _turretcore_2 (`self.turretCore`))
  (if isRelative
    (`SceneComponent.K2_SetRelativeRotation` _turretcore_2 (`KismetMathLibrary.RLerp` (`SceneComponent.RelativeRotation` _turretcore_2) B (* (`GameplayStatics.GetWorldDeltaSeconds`) 20.0)) false false)
    (else
      (`SceneComponent.K2_SetWorldRotation` _turretcore (`KismetMathLibrary.RLerp` (`SceneComponent.K2_GetComponentRotation` _turretcore) B (* (`GameplayStatics.GetWorldDeltaSeconds`) 20.0)) false false))))

(fn `UserConstructionScript`
  (bind _capsule (`self.Capsule`))
  (`CapsuleComponent.SetCapsuleHalfHeight` _capsule (`self.range`) true)
  (`CapsuleComponent.SetCapsuleRadius` _capsule (`self.radius`) true)
  (`self.changeColor` (`self.color`)))