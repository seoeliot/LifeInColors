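; Turret projectile that homes onto a target and applies an effect chosen by its color on arrival or hit.
; With a valid target, a timeline lerps it to the target's location; otherwise it simulates physics, gets a forward impulse and expires after a short delay.
; Yellow launches characters along the bullet's forward vector, Green and None destroy the target, and Red only destroys the bullet.
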(event `self.ReceiveBeginPlay`
  (bind _sphere (`self.Sphere`))
  (`/Engine/EditorBlueprintResources/StandardMacros.IsValid` (`self.target`)
    (:`Is Valid`
      (bind (_direction _newtrack_0) (`Timeline|Timeline_0`)
        (:`Update`
          (`self.K2_SetActorLocation` (`KismetMathLibrary.VLerp` (`SceneComponent.K2_GetComponentLocation` (`self.Sphere`)) (`self.K2_GetActorLocation` (`self.target`)) _newtrack_0)))
        (:`Finished`
          (`self.On Target Reached` (`self.target`)))))
    (:`Is Not Valid`
      (`PrimitiveComponent.SetSimulatePhysics` (`self.Sphere`) true)
      (`PrimitiveComponent.AddImpulse` _sphere (* (`SceneComponent.GetForwardVector` _sphere) (`KismetMathLibrary.Conv_DoubleToVector` 1000.0)) "None" false)
      (`KismetSystemLibrary.Delay` 1.0)
      (`self.K2_DestroyActor`))))

(event `On Target Reached`
  (params (target :type "Actor Object Reference"))
  (switch `/Game/MyGame/Data/EnumColor` (`self.color`)
    (:`NewEnumerator1`
      (if (`self.ActorHasTag` target (`self.Tag`))
        (`self.K2_DestroyActor`))
      (`self.K2_DestroyActor` :!label _label))
    (:`NewEnumerator2`
      (bind _ascharacter (cast `Character` target))
      (`Character.LaunchCharacter` _ascharacter (* (`SceneComponent.GetForwardVector` (`self.Sphere`)) (`KismetMathLibrary.Conv_DoubleToVector` 500.0)) false false)
      (goto _label))
    (:`NewEnumerator3`
      (`/Engine/EditorBlueprintResources/StandardMacros.IsValid` target :!label _label_2
        (:`Is Valid`
          (`self.K2_DestroyActor` target)
          (`self.K2_DestroyActor`))))
    (:`NewEnumerator4`
      (goto _label_2))))

(event `self.Sphere.OnComponentHit`
  (params (HitComponent :type "PrimitiveComponent Object Reference") (OtherActor :type "Actor Object Reference") (OtherComp :type "PrimitiveComponent Object Reference") (NormalImpulse :type "Vector Structure") (Hit :type "HitResult Structure (by ref)"))
  (`self.On Target Reached` OtherActor))

(fn `UserConstructionScript`)