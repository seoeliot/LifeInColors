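; Paintable jukebox whose color decides both its look and the song it plays.
; The construction script and ChangeColor apply the color's material set to the top and bottom meshes.
; ChangeColor fires a dispatcher from inside its material loop, triggering the handler that also runs at BeginPlay.
; That handler shows and activates only the matching colored component and plays that color's song, or hub music when None.
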(event `self.ReceiveBeginPlay`
  (`self.BeginFunction`)
  (add `self.NewEventDispatcher_0` (delegate `EventOnChangeColor`))
  (`self.EventOnChangeColor`))

(event `EventOnChangeColor`
  (bind _jukeboxgreen (`self.JukeBoxGreen`))
  (bind _jukeboxyellow (`self.JukeBoxYellow`))
  (bind _jukeboxred (`self.JukeboxRed`))
  (bind _jukeboxblue (`self.JukeBoxBlue`))
  (`ActorComponent.Deactivate` (`self.JukeBoxBlue`))
  (`ActorComponent.Deactivate` (`self.JukeboxRed`))
  (`ActorComponent.Deactivate` (`self.JukeBoxGreen`))
  (`ActorComponent.Deactivate` (`self.JukeBoxYellow`))
  (`SceneComponent.SetVisibility` (`self.JukeboxRed`) false false)
  (`SceneComponent.SetVisibility` (`self.JukeBoxGreen`) false false)
  (`SceneComponent.SetVisibility` (`self.JukeBoxYellow`) false false)
  (`SceneComponent.SetVisibility` (`self.JukeBoxBlue`) false false)
  (switch `/Game/MyGame/Data/EnumColor` (`self.EnumColor`)
    (:`NewEnumerator0`
      (`AudioComponent.SetSound` (`self.Audio`) "/Game/MyGame/Sound/BlueSong.BlueSong")
      (`ActorComponent.Activate` _jukeboxblue false)
      (`SceneComponent.SetVisibility` _jukeboxblue true false)
      (`AudioComponent.Play` (`self.Audio`) 0.0 :!label _label))
    (:`NewEnumerator1`
      (`AudioComponent.SetSound` (`self.Audio`) "/Game/MyGame/Sound/RedSong.RedSong")
      (`ActorComponent.Activate` _jukeboxred false)
      (`SceneComponent.SetVisibility` _jukeboxred true false)
      (goto _label))
    (:`NewEnumerator2`
      (`AudioComponent.SetSound` (`self.Audio`) "/Game/MyGame/Sound/JauneSong.JauneSong")
      (`ActorComponent.Activate` _jukeboxyellow false)
      (`SceneComponent.SetVisibility` _jukeboxyellow true false)
      (goto _label))
    (:`NewEnumerator3`
      (`AudioComponent.SetSound` (`self.Audio`) "/Game/MyGame/Sound/VertSong.VertSong")
      (`ActorComponent.Activate` _jukeboxgreen false)
      (`SceneComponent.SetVisibility` _jukeboxgreen true false)
      (goto _label))
    (:`NewEnumerator4`
      (`AudioComponent.SetSound` (`self.Audio`) "/Game/MyGame/Sound/MusicHub.MusicHub")
      (`AudioComponent.Play` (`self.Audio`) 0.0))))

(fn `ChangeColor`
  (params (newColor :type "/Game/MyGame/Data/EnumColor Enum" :default "NewEnumerator0"))
  (bind (_mat_none _mat_blue _mat_green _mat_yellow _mat_red) (break `/Game/MyGame/Data/StructColorText` (`self.StructColor`)))
  (set `self.EnumColor` newColor)
  (for _array_element (select `/Game/MyGame/Data/EnumColor` (`self.EnumColor`) :`NewEnumerator0` _mat_blue :`NewEnumerator1` _mat_red :`NewEnumerator2` _mat_yellow :`NewEnumerator3` _mat_green :`NewEnumerator4` _mat_none)
    (`PrimitiveComponent.SetMaterial` (`self.JukeboxBas`) 0 _array_element)
    (`PrimitiveComponent.SetMaterial` (`self.JukeboxHaut`) 0 _array_element)
    (`self.NewEventDispatcher_0`)))

(fn `ResetColor`)

(fn `UserConstructionScript`
  (bind (_mat_none _mat_blue _mat_green _mat_yellow _mat_red) (break `/Game/MyGame/Data/StructColorText` (`self.StructColor`)))
  (for (_array_element _array_index) (select `/Game/MyGame/Data/EnumColor` (`self.EnumColor`) :`NewEnumerator0` _mat_blue :`NewEnumerator1` _mat_red :`NewEnumerator2` _mat_yellow :`NewEnumerator3` _mat_green :`NewEnumerator4` _mat_none)
    (`PrimitiveComponent.SetMaterial` (`self.JukeboxHaut`) _array_index _array_element)
    (`PrimitiveComponent.SetMaterial` (`self.JukeboxBas`) _array_index _array_element)))