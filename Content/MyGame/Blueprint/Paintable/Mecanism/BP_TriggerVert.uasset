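; BP_TriggerVert is an interactable pickup that unlocks the green color and sends the player to another level.
; A sphere overlap by BP_FirstPerson shows an interact prompt widget.
; On interact, it plays a sound, shows the unlock widget, fades to black, blocks movement and sets the player's current-level value.
; After a delay, it registers the color unlock in GI_Main and opens the referenced level.
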(event `self.OnInteract`
  (`GameplayStatics.PlaySound2D` "/Game/MyGame/Sound/SoundEffect/Unlock.Unlock" 1.0 1.0 0.0 null null)
  (bind _returnvalue (`|CreateWidget` "/Game/MyGame/UI_HUD/WB_Tutos/GreenUnlock.GreenUnlock_C"))
  (`UserWidget.AddToViewport` _returnvalue 0)
  (`KismetSystemLibrary.Delay` 0.2)
  (`PlayerCameraManager.StartCameraFade` (`GameplayStatics.GetPlayerCameraManager` 0) 0.0 1.0 2.0 (struct :`A` 1.0) true true)
  (`Controller.SetIgnoreMoveInput` (`GameplayStatics.GetPlayerController` 0) true)
  (bind _asbp_first_person (cast `/Game/MyGame/Blueprint/BP_FirstPerson/BP_FirstPerson` (`GameplayStatics.GetPlayerCharacter` 0)))
  (set `/Game/MyGame/Blueprint/BP_FirstPerson/BP_FirstPerson.LevelActuel` "/Game/MyGame/LD/Level_1Retour.Level_1Retour" _asbp_first_person)
  (`KismetSystemLibrary.Delay` 2.0)
  (bind _asgi_main (cast `/Game/MyGame/GameInstance/GI_Main` (`GameplayStatics.GetGameInstance`)))
  (`/Game/MyGame/GameInstance/GI_Main.EventUnlockColor` _asgi_main 3)
  (`GameplayStatics.OpenLevelBySoftObjectPtr` (`self.Level`)))

(event `self.Sphere1.OnComponentBeginOverlap`
  (params (OverlappedComponent :type "PrimitiveComponent Object Reference") (OtherActor :type "Actor Object Reference") (OtherComp :type "PrimitiveComponent Object Reference") (OtherBodyIndex :type Integer) (bFromSweep :type Boolean) (SweepResult :type "HitResult Structure (by ref)"))
  (cast `/Game/MyGame/Blueprint/BP_FirstPerson/BP_FirstPerson` OtherActor)
  (bind _returnvalue (`|CreateWidget` "/Game/MyGame/UI_HUD/Etointeract.Etointeract_C"))
  (`UserWidget.AddToViewport` _returnvalue 0))

(fn `OnChangeColor`)

(fn `UserConstructionScript`)