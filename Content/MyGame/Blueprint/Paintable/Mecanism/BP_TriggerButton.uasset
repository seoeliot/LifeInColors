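; Paintable trigger button whose press behavior depends on its current paint color.
; On interact it pushes immediately when blue, red or unpainted, or after a delay when green, while yellow pushes itself repeatedly from Tick.
; Delayed pushes recheck the color first, and a Pushable flag, reset on color change, blocks overlapping interactions.
; Each push calls the begin trigger, then the end trigger a second later, re-arming the button.
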(event `self.ReceiveBeginPlay`
  (add `self.EndTrigger` (delegate `EndTrigger_Event`)))

(event `self.ReceiveTick`
  (params (DeltaSeconds :type "Float (single-precision)"))
  (switch `/Game/MyGame/Data/EnumColor` (`self.PaintColor`)
    (:`NewEnumerator2`
      (if (`self.bPushable`)
        (`KismetSystemLibrary.Delay` 2.0)
        (`self.CheckColor` "NewEnumerator2"
          (:`True`
            (`self.PushButton`)))))))

(event `EndTrigger_Event`
  (`KismetSystemLibrary.PrintString` "Push button"))

(event `self.OnInteract`
  (bind _bpushable (`self.bPushable`))
  (if _bpushable
    (if (and _bpushable (`|EnumInequality` (`self.PaintColor`) "NewEnumerator2"))
      (set `self.bPushable` false))
    (switch `/Game/MyGame/Data/EnumColor` (`self.PaintColor`)
      (:`NewEnumerator0`
        (`self.PushButton`))
      (:`NewEnumerator1`
        (`self.PushButton`))
      (:`NewEnumerator3`
        (`KismetSystemLibrary.Delay` 3.0)
        (`self.CheckColor` "NewEnumerator3"
          (:`True`
            (`self.PushButton`))))
      (:`NewEnumerator4`
        (`self.PushButton`)))))

(event `PushButton`
  (`self.BeginTrigger`)
  (`KismetSystemLibrary.Delay` 1.0)
  (`self.EndTrigger`)
  (set `self.bPushable` true))

(fn `OnChangeColor`
  (set `self.bPushable` true))

(fn `UserConstructionScript`
  (locals (L_TargetArray :type "Array of /Game/MyGame/Blueprint/Paintable/Mecanism/BP_Activable Object Reference") (L_AllActivables :type "Set of /Game/MyGame/Blueprint/Paintable/Mecanism/BP_Activable Object Reference")))