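; Paintable conveyor belt that pushes tagged player and cube actors along its forward vector, with behavior set by its color.
; Color swaps materials and sets belt and shader speed: blue stops, red accelerates, green reverses, yellow or none runs normally.
; Tick applies impulses to actors tracked by box overlap, skipping blue cubes; brief physics toggles kill cube momentum on entry, exit or stop.
; Yellow belts also bounce the player upward on hit.
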(event `self.ReceiveTick`
  (params (DeltaSeconds :type "Float (single-precision)"))
  (bind _returnvalue (* (* (`self.GetActorForwardVector`) (`self.NewSpeed`)) 100.0))
  (for _array_element (`self.ActorOverlaping`)
    ;[1 1 1] Déplacement cube
    (bind _asbp_paintable_cube (cast `/Game/MyGame/Blueprint/Paintable/BP_PaintableCube` _array_element)
      (:`then`
        (if (`|EnumInequality` "NewEnumerator0" (`/Game/MyGame/Blueprint/Paintable/BP_PaintableCube.Color` _asbp_paintable_cube))
          (`PrimitiveComponent.AddImpulse` (`/Game/MyGame/Blueprint/Paintable/BP_PaintableCube.StaticMesh` _asbp_paintable_cube) _returnvalue "None" false)))
      (:`CastFailed`
        ;[1 1 1] Déplacement joueur
        (bind _asbp_first_person (cast `/Game/MyGame/Blueprint/BP_FirstPerson/BP_FirstPerson` _array_element))
        (`CharacterMovementComponent.AddImpulse` (`Character.CharacterMovement` _asbp_first_person) (/ _returnvalue 3.0) true)))))

(event `self.Box.OnComponentBeginOverlap`
  (params (OverlappedComponent :type "PrimitiveComponent Object Reference") (OtherActor :type "Actor Object Reference") (OtherComp :type "PrimitiveComponent Object Reference") (OtherBodyIndex :type Integer) (bFromSweep :type Boolean) (SweepResult :type "HitResult Structure (by ref)"))
  ;[1 1 1] Entré et sortie du tapis
  (bind _asgi_main (cast `/Game/MyGame/GameInstance/GI_Main` (`GameplayStatics.GetGameInstance`)))
  (if (`self.ActorHasTag` OtherActor (`/Game/MyGame/GameInstance/GI_Main.TagNameTapisRoulant` _asgi_main))
    (`KismetArrayLibrary.Array_AddUnique` (`self.ActorOverlaping`) OtherActor)
    ;[0.5417 0.1752 0] fin / entré tapis
    (bind _asbp_paintable_cube (cast `/Game/MyGame/Blueprint/Paintable/BP_PaintableCube` OtherActor))
    (`KismetSystemLibrary.Delay` 0.5)
    (`PrimitiveComponent.SetSimulatePhysics` (`/Game/MyGame/Blueprint/Paintable/BP_PaintableCube.StaticMesh` _asbp_paintable_cube) false)
    (`KismetSystemLibrary.Delay` 0.1)
    (`PrimitiveComponent.SetSimulatePhysics` (`/Game/MyGame/Blueprint/Paintable/BP_PaintableCube.StaticMesh` _asbp_paintable_cube) true)))

(event `self.Box.OnComponentEndOverlap`
  (params (OverlappedComponent :type "PrimitiveComponent Object Reference") (OtherActor :type "Actor Object Reference") (OtherComp :type "PrimitiveComponent Object Reference") (OtherBodyIndex :type Integer))
  ;[1 1 1] Entré et sortie du tapis
  (bind _asgi_main (cast `/Game/MyGame/GameInstance/GI_Main` (`GameplayStatics.GetGameInstance`)))
  (if (`self.ActorHasTag` OtherActor (`/Game/MyGame/GameInstance/GI_Main.TagNameTapisRoulant` _asgi_main))
    (`KismetArrayLibrary.Array_RemoveItem` (`self.ActorOverlaping`) OtherActor)
    ;[0.5417 0.1752 0] fin / entré tapis
    (bind _asbp_paintable_cube (cast `/Game/MyGame/Blueprint/Paintable/BP_PaintableCube` OtherActor))
    (`KismetSystemLibrary.Delay` 0.1)
    (`PrimitiveComponent.SetSimulatePhysics` (`/Game/MyGame/Blueprint/Paintable/BP_PaintableCube.StaticMesh` _asbp_paintable_cube) false)
    (`KismetSystemLibrary.Delay` 0.1)
    (`PrimitiveComponent.SetSimulatePhysics` (`/Game/MyGame/Blueprint/Paintable/BP_PaintableCube.StaticMesh` _asbp_paintable_cube) true)))

(event `OnChangeCouleur`
  ;[1 1 1] Color Change
  (switch `/Game/MyGame/Data/EnumColor` (`self.Color`)
    (:`NewEnumerator0`
      (bind _output_get (set `self.NewSpeed` 0.0))
      (`MeshComponent.SetScalarParameterValueOnMaterials` (`self.StaticMesh`) "Speed" _output_get)
      ;[0 0.1401 1] Le bleu stopp les cube qui bougent sur la tapis
      (if (> (`KismetArrayLibrary.Array_Length` (`self.ActorOverlaping`)) 0)
        (for _array_element (`self.ActorOverlaping`)
          (bind _asbp_paintable_cube (cast `/Game/MyGame/Blueprint/Paintable/BP_PaintableCube` _array_element))
          (`KismetSystemLibrary.Delay` 0.1)
          (`PrimitiveComponent.SetSimulatePhysics` (`/Game/MyGame/Blueprint/Paintable/BP_PaintableCube.StaticMesh` _asbp_paintable_cube) false)
          (`KismetSystemLibrary.Delay` 0.1)
          (`PrimitiveComponent.SetSimulatePhysics` (`/Game/MyGame/Blueprint/Paintable/BP_PaintableCube.StaticMesh` _asbp_paintable_cube) true))))
    (:`NewEnumerator1`
      (bind _output_get_2 (set `self.NewSpeed` (* (`self.Speed`) 3.5)))
      (`MeshComponent.SetScalarParameterValueOnMaterials` (`self.StaticMesh`) "Speed" _output_get_2))
    (:`NewEnumerator2`
      (bind _output_get_3 (set `self.NewSpeed` (`self.Speed`) :!label _label))
      (`MeshComponent.SetScalarParameterValueOnMaterials` (`self.StaticMesh`) "Speed" _output_get_3))
    (:`NewEnumerator3`
      (bind _output_get_4 (set `self.NewSpeed` (* (`self.Speed`) -1.0)))
      (`MeshComponent.SetScalarParameterValueOnMaterials` (`self.StaticMesh`) "Speed" _output_get_4))
    (:`NewEnumerator4`
      (goto _label))))

(event `self.StaticMesh.OnComponentHit`
  (params (HitComponent :type "PrimitiveComponent Object Reference") (OtherActor :type "Actor Object Reference") (OtherComp :type "PrimitiveComponent Object Reference") (NormalImpulse :type "Vector Structure") (Hit :type "HitResult Structure (by ref)"))
  ;[1 0.8173 0] Rebondis
  (if (`|EnumEquality` (`self.Color`) "NewEnumerator2")
    (bind _asbp_first_person (cast `/Game/MyGame/Blueprint/BP_FirstPerson/BP_FirstPerson` OtherActor))
    (bind (_returnvalue_x _returnvalue_y _returnvalue_z) (`KismetMathLibrary.BreakVector` (`SceneComponent.GetComponentVelocity` (`Actor.RootComponent` _asbp_first_person))))
    (`Character.LaunchCharacter` _asbp_first_person (`KismetMathLibrary.MakeVector` 0.0 0.0 (* (`KismetMathLibrary.FClamp` _returnvalue_z -4200.0 -420.0) -1.0)) false true)))

(fn `ChangeColor`
  (params (Couleur :type "/Game/MyGame/Data/EnumColor Enum" :default "NewEnumerator0"))
  (bind (_mat_none _mat_blue _mat_green _mat_yellow _mat_red) (break `/Game/MyGame/Data/StructColorText` (`self.ColorTextures`)))
  (set `self.Color` Couleur)
  (for (_array_element _array_index) (select `/Game/MyGame/Data/EnumColor` (`self.Color`) :`NewEnumerator0` _mat_blue :`NewEnumerator1` _mat_red :`NewEnumerator2` _mat_yellow :`NewEnumerator3` _mat_green :`NewEnumerator4` _mat_none)
    (`PrimitiveComponent.SetMaterial` (`self.StaticMesh`) _array_index _array_element)
    (`self.OnChangeCouleur`)))

(fn `UserConstructionScript`
  (`|ExecutionSequence`
    (:`then_0`
      (`MeshComponent.SetScalarParameterValueOnMaterials` (`self.StaticMesh`) "Speed" (`self.Speed`)))
    (:`then_1`
      (`self.ChangeColor` (`self.Color`)))))