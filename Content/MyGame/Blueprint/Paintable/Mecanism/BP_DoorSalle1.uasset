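; BP_DoorSalle1 is a door actor that swings between closed and open orientations according to its Open flag.
; BeginPlay caches the starting rotation as closed and derives the open yaw by subtracting 90 degrees.
; Tick passes through a short Delay, then snaps the actor to the matching rotation without interpolation.
; Nothing in this Blueprint sets Open.
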(event `self.ReceiveTick`
  (params (DeltaSeconds :type "Float (single-precision)"))
  (`KismetSystemLibrary.Delay` 0.1)
  (if (`self.Open`)
    (`self.K2_SetActorRotation` (`KismetMathLibrary.MakeRotator` (`self.RotaX`) (`self.RotaY`) (`self.Rotaouvert`)))
    (else
      (`self.K2_SetActorRotation` (`KismetMathLibrary.MakeRotator` (`self.RotaX`) (`self.RotaY`) (`self.RotaZ`))))))

(event `self.ReceiveBeginPlay`
  (bind (_returnvalue_roll _returnvalue_pitch _returnvalue_yaw) (`KismetMathLibrary.BreakRotator` (`self.K2_GetActorRotation`)))
  (set `self.RotaX` _returnvalue_roll)
  (set `self.RotaY` _returnvalue_pitch)
  (set `self.RotaZ` _returnvalue_yaw)
  (set `self.Rotaouvert` (+ _returnvalue_yaw -90.0)))

(fn `UserConstructionScript`)