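; Two-state lever, likely for room 1 (Salle1), that fires triggers when the player interacts with it.
; OnInteract flips Up, mirrors it to IsActivated, swaps the two cube meshes, plays a click and calls EndTrigger when up, BeginTrigger when down.
; Construction previews the initial state, and BeginPlay reapplies it, including sound and trigger.
; Sphere1 overlap by BP_FirstPerson adds an Etointeract prompt widget, never removed here.
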(event `self.ReceiveBeginPlay`
  (if (`self.Up`)
    (`SceneComponent.SetVisibility` (`self.Cube2`) true false :!label _label)
    (`SceneComponent.SetVisibility` (`self.Cube1`) false false)
    (bind _output_get (set `self.Up` true))
    (set `self.bIsActivated` _output_get)
    (`GameplayStatics.PlaySound2D` "/Game/MyGame/Sound/Button_Plate_Click__Minecraft_Sound__-_Sound_Effect_for_editing.Button_Plate_Click__Minecraft_Sound__-_Sound_Effect_for_editing" 1.0 1.0 0.0 null null)
    (`self.EndTrigger`)
    (else
      (`SceneComponent.SetVisibility` (`self.Cube2`) false false :!label _label_2)
      (`SceneComponent.SetVisibility` (`self.Cube1`) true false)
      (bind _output_get_2 (set `self.Up` false))
      (set `self.bIsActivated` _output_get_2)
      (`GameplayStatics.PlaySound2D` "/Game/MyGame/Sound/Button_Plate_Click__Minecraft_Sound__-_Sound_Effect_for_editing.Button_Plate_Click__Minecraft_Sound__-_Sound_Effect_for_editing" 1.0 1.0 0.0 null null)
      (`self.BeginTrigger`))))

(event `self.OnInteract`
  (if (`self.Up`)
    (goto _label_2)
    (else
      (goto _label))))

(event `self.Sphere1.OnComponentBeginOverlap`
  (params (OverlappedComponent :type "PrimitiveComponent Object Reference") (OtherActor :type "Actor Object Reference") (OtherComp :type "PrimitiveComponent Object Reference") (OtherBodyIndex :type Integer) (bFromSweep :type Boolean) (SweepResult :type "HitResult Structure (by ref)"))
  (cast `/Game/MyGame/Blueprint/BP_FirstPerson/BP_FirstPerson` OtherActor)
  (bind _returnvalue (`|CreateWidget` "/Game/MyGame/UI_HUD/Etointeract.Etointeract_C"))
  (`UserWidget.AddToViewport` _returnvalue 0))

(fn `OnChangeColor`)

(fn `UserConstructionScript`
  (if (`self.Up`)
    (set `self.bIsActivated` true)
    (`SceneComponent.SetVisibility` (`self.Cube2`) true false)
    (`SceneComponent.SetVisibility` (`self.Cube1`) false false)
    (else
      (set `self.bIsActivated` false)
      (`SceneComponent.SetVisibility` (`self.Cube2`) false false)
      (`SceneComponent.SetVisibility` (`self.Cube1`) true false))))