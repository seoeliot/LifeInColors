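; Pedestal actor that shows which colors the player has unlocked, with five colored cylinders, each paired with a component it activates.
; Every Tick it reads the UnlockedColor boolean array from the GI_Main game instance.
; For each unlocked index it activates the matching pedestal component and sets that cylinder's material to blue, red, yellow, green or the base material for white.
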(event `self.ReceiveTick`
  (params (DeltaSeconds :type "Float (single-precision)"))
  (bind _asgi_main (cast `/Game/MyGame/GameInstance/GI_Main` (`GameplayStatics.GetGameInstance`)))
  (for (_array_element _array_index) (`/Game/MyGame/GameInstance/GI_Main.UnlockedColor` _asgi_main)
    (if _array_element
      (switch `int` _array_index
        (:`0`
          (`ActorComponent.Activate` (`self.PiedestalBleu`) false)
          (`PrimitiveComponent.SetMaterial` (`self.CylinderBleu`) 0 "/Game/MyGame/Materials/Mat_Blue.Mat_Blue"))
        (:`1`
          (`ActorComponent.Activate` (`self.PiedestalRouge`) false)
          (`PrimitiveComponent.SetMaterial` (`self.CylinderRouge`) 0 "/Game/MyGame/Materials/Mat_Red.Mat_Red"))
        (:`2`
          (`ActorComponent.Activate` (`self.PiedestalPastis`) false)
          (`PrimitiveComponent.SetMaterial` (`self.CylinderJaune`) 0 "/Game/MyGame/Materials/Mat_Yellow.Mat_Yellow"))
        (:`3`
          (`ActorComponent.Activate` (`self.PiedestalVert`) false)
          (`PrimitiveComponent.SetMaterial` (`self.CylinderVert`) 0 "/Game/MyGame/Materials/Mat_Green.Mat_Green"))
        (:`4`
          (`ActorComponent.Activate` (`self.PiedestalBlanc`) false)
          (`PrimitiveComponent.SetMaterial` (`self.CylinderBlanc`) 0 "/Game/UE5/FPWeapon/Materials/BaseMaterial.BaseMaterial"))))))

(fn `UserConstructionScript`)