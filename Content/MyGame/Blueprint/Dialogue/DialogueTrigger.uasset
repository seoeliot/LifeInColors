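; DialogueTrigger is a level trigger that starts a dialogue in the game when a tagged actor overlaps it.
; On overlap with an actor tagged TriggerDial, it passes its Dialogue data to the GM_InGame game mode's EventDialogue.
; An EstActivé flag makes it fire only once, and when Cinématique is enabled it also sets CinémaTrigger to true.
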(event `self.ReceiveActorBeginOverlap`
  (params (OtherActor :type "Actor Object Reference"))
  (if (`self.ActorHasTag` OtherActor "TriggerDial")
    (if (not (`self.EstActivé`))
      (bind _asgm_in_game (cast `/Game/MyGame/GameInstance/GM_InGame` (`GameplayStatics.GetGameMode`)))
      (`/Game/MyGame/GameInstance/GM_InGame.EventDialogue` _asgm_in_game (`self.Dialogue`))
      (set `self.EstActivé` true)
      (if (`self.Cinématique`)
        (set `self.CinémaTrigger` true)))))

(fn `UserConstructionScript`)