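; Tutorial trigger that unlocks a color, apparently red, once the first-person player has a color gun.
; Box overlap and Tick share one chain, gated on a specific GI_Main progression state and a valid color gun on the overlapping BP_FirstPerson.
; It shows the RedUnlock widget, advances progression, and fires unlock events on the game instance and GestionDeProgression.
; It then notifies the player pawn's color gun and destroys itself.
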(event `self.ReceiveTick`
  (params (DeltaSeconds :type "Float (single-precision)"))
  (bind _asgi_main (cast `/Game/MyGame/GameInstance/GI_Main` (`GameplayStatics.GetGameInstance`) :!label _label))
  (if (`|EnumEquality` (`/Game/MyGame/GameInstance/GI_Main.ProgressionState` _asgi_main) "NewEnumerator0")
    (bind _asbp_first_person (cast `/Game/MyGame/Blueprint/BP_FirstPerson/BP_FirstPerson` (stale `self.Box.OnComponentBeginOverlap` OtherActor)))
    (`/Engine/EditorBlueprintResources/StandardMacros.IsValid` (`/Game/MyGame/Blueprint/BP_FirstPerson/BP_FirstPerson.ColorgunReference` _asbp_first_person)
      (:`Is Valid`
        (bind _returnvalue (`|CreateWidget` "/Game/MyGame/UI_HUD/WB_Tutos/RedUnlock.RedUnlock_C"))
        (`UserWidget.AddToViewport` _returnvalue 0)
        (bind _asgi_main_2 (cast `/Game/MyGame/GameInstance/GI_Main` (`GameplayStatics.GetGameInstance`)))
        (set `/Game/MyGame/GameInstance/GI_Main.ProgressionState` "NewEnumerator6" _asgi_main_2)
        (`/Game/MyGame/GameInstance/GI_Main.EventUnlockColor` _asgi_main_2 1)
        (`/Game/MyGame/Blueprint/GestionDeProgression.DeblocageEvent` (`self.GestionDeProgression`))
        (bind _asbp_first_person_2 (cast `/Game/MyGame/Blueprint/BP_FirstPerson/BP_FirstPerson` (`GameplayStatics.GetPlayerPawn` 0)))
        (bind _colorgunreference (`/Game/MyGame/Blueprint/BP_FirstPerson/BP_FirstPerson.ColorgunReference` _asbp_first_person_2))
        (`/Engine/EditorBlueprintResources/StandardMacros.IsValid` _colorgunreference
          (:`Is Valid`
            (`/Game/MyGame/Blueprint/BP_FirstPerson/BP_Colorgun.EventUnlockColor` _colorgunreference)
            (`self.K2_DestroyActor`)))))))

(event `self.Box.OnComponentBeginOverlap`
  (params (OverlappedComponent :type "PrimitiveComponent Object Reference") (OtherActor :type "Actor Object Reference") (OtherComp :type "PrimitiveComponent Object Reference") (OtherBodyIndex :type Integer) (bFromSweep :type Boolean) (SweepResult :type "HitResult Structure (by ref)"))
  (goto _label))

(fn `UserConstructionScript`)