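; Swing Blueprint (balançoire) that rocks two static meshes back and forth in opposite directions.
; An endless Delay loop started on BeginPlay flips the Aller flag at a fixed interval.
; Each Tick adds a fixed local rotation to both meshes, with the sign set by Aller.
; The rotation step is not scaled by delta time, so the swing arc depends on frame rate.
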(event `self.ReceiveBeginPlay`
  (`KismetSystemLibrary.Delay` 1.5 :!label _label)
  (set `self.Aller` true)
  (`KismetSystemLibrary.Delay` 1.5)
  (set `self.Aller` false)
  (goto _label))

(event `self.ReceiveTick`
  (params (DeltaSeconds :type "Float (single-precision)"))
  (bind _staticmesh1 (`self.StaticMesh1`))
  (bind _staticmesh (`self.StaticMesh`))
  (`|ExecutionSequence`
    (:`then_0`
      (if (`self.Aller`)
        (`SceneComponent.K2_AddLocalRotation` _staticmesh (struct :`Roll` 1.0) false false)
        (else
          (`SceneComponent.K2_AddLocalRotation` _staticmesh (struct :`Roll` -1.0) false false))))
    (:`then_1`
      (if (`self.Aller`)
        (`SceneComponent.K2_AddLocalRotation` _staticmesh1 (struct :`Roll` -1.0) false false)
        (else
          (`SceneComponent.K2_AddLocalRotation` _staticmesh1 (struct :`Roll` 1.0) false false))))))

(fn `UserConstructionScript`)