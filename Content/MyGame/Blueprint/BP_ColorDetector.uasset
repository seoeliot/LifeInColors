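; Color-coded detector that activates when a paintable cube of the matching color is within its capsule and in line of sight.
; Each Tick it resets and fires the end trigger, then re-checks overlapping cubes and fires the begin trigger on a match.
; Sight uses a debug-drawn sphere trace that ignores the parent platform.
; The construction script sets mesh and decal materials from the chosen color.
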(event `self.ReceiveTick`
  (params (DeltaSeconds :type "Float (single-precision)"))
  (set `self.bIsActivated` false)
  (`self.EndTrigger`)
  (for _array_element (`PrimitiveComponent.GetOverlappingActors` (`self.Capsule`) null)
    (bind _asbp_paintable_cube (cast `/Game/MyGame/Blueprint/Paintable/BP_PaintableCube` _array_element))
    (bind _bobjecthit (`self.Check Object in Sight` _asbp_paintable_cube))
    (if (and _bobjecthit (`|EnumEquality` (`/Game/MyGame/Blueprint/Paintable/BP_PaintableCube.Color` _asbp_paintable_cube) (`self.Color`)))
      (set `self.bIsActivated` true)
      (`self.BeginTrigger`)
      (`KismetSystemLibrary.PrintString` "Hit color !" true true (struct :`G` 0.66 :`B` 1.0 :`A` 1.0) 0.0))))

(fn `Check Object in Sight`
  (params (other :type "Actor Object Reference"))
  (returns (bObjectHit :type Boolean))
  (locals (localOther :type "Actor Object Reference"))
  (bind _output_get (set `local.localOther` other))
  (bind _outhit (`KismetSystemLibrary.SphereTraceSingle` (`SceneComponent.K2_GetComponentLocation` (`self.StaticMesh`)) (`SceneComponent.K2_GetComponentLocation` (`Actor.RootComponent` _output_get)) 50.0 "TraceTypeQuery1" false (`|MakeArray` (`self.parentPlatform`)) "ForOneFrame"))
  (bind (_bblockinghit _binitialoverlap _time _distance _location _impactpoint _normal _impactnormal _physmat _hitactor) (`GameplayStatics.BreakHitResult` _outhit))
  (`KismetSystemLibrary.PrintString` (`KismetSystemLibrary.GetDisplayName` _hitactor) true true (struct :`G` 0.66 :`B` 1.0 :`A` 1.0) 0.0)
  (return (== _hitactor (`local.localOther`))))

(fn `UserConstructionScript`
  (`PrimitiveComponent.SetMaterial` (`self.StaticMesh`) 0 (select `/Game/MyGame/Data/EnumColor` (`self.Color`) :`NewEnumerator0` "/Game/MyGame/Materials/Mat_Blue.Mat_Blue" :`NewEnumerator1` "/Game/MyGame/Materials/Mat_Red.Mat_Red" :`NewEnumerator2` "/Game/MyGame/Materials/Mat_Yellow.Mat_Yellow" :`NewEnumerator3` "/Game/MyGame/Materials/Mat_Green.Mat_Green" :`NewEnumerator4` "/Game/UE5/FPWeapon/Materials/BaseMaterial.BaseMaterial" :!type "MaterialInterface Object Reference"))
  (`DecalComponent.SetDecalMaterial` (`self.Decal`) (select `/Game/MyGame/Data/EnumColor` (`self.Color`) :`NewEnumerator0` "/Game/MyGame/Materials/Mat_DecalBlue.Mat_DecalBlue" :`NewEnumerator1` "/Game/MyGame/Materials/Mat_DecalRed.Mat_DecalRed" :`NewEnumerator2` "/Game/MyGame/Materials/Mat_DecalYellow.Mat_DecalYellow" :`NewEnumerator3` "/Game/MyGame/Materials/Mat_DecalGreen.Mat_DecalGreen" :`NewEnumerator4` "/Game/UE5/FPWeapon/Materials/BaseMaterial.BaseMaterial" :!type "MaterialInterface Object Reference")))