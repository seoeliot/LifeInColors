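; Moving color platform that travels between two points offset from its placed location and can change color.
; A timeline lerps the mesh, with speed set through CustomTimeDilation; PingPong reverses it, and restarting forward requires enough triggers.
; The color enum selects material sets at construction and in ChangeColor, which also fires an event dispatcher.
; Construction snaps an attached child actor to the mesh with offsets and registers the platform as parent of a BP_ColorDetector child.
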(event `self.ReceiveBeginPlay`
  (set `self.CustomTimeDilation` (`self.speed`))
  (`self.BeginFunction`)
  (set `self.BeginLoc` (+ (`self.K2_GetActorLocation`) (`self.BeginLoc`)))
  (set `self.EndLoc` (+ (`self.EndLoc`) (`self.K2_GetActorLocation`)))
  (`TimelineComponent.SetNewTime` (`self.Timeline_0`) (`self.Newtime`))
  (switch `ETimelineDirection` (stale _direction)
    (:`Forward`
      (bind (_direction _newtrack_0) (`Timeline|Timeline_0` :!label _label)
        (:`Update`
          (`SceneComponent.K2_SetWorldLocation` (`self.StaticMesh`) (`KismetMathLibrary.VLerp` (`self.BeginLoc`) (`self.EndLoc`) _newtrack_0) false false))
        (:`Finished`
          (switch `ETimelineDirection` _direction
            (:`Forward`
              (if (`self.bPingPong`)
                (goto _label :!via `Reverse`)))
            (:`Backward`
              (`self.CheckEnergy`
                (:`enoughEnergy`
                  (goto _label))))))))
    (:`Backward`
      (goto _label :!via `Reverse`))))

(fn `ChangeColor`
  (params (newColor :type "/Game/MyGame/Data/EnumColor Enum" :default "NewEnumerator0"))
  (bind (_mat_none _mat_blue _mat_green _mat_yellow _mat_red) (break `/Game/MyGame/Data/StructColorText` (`self.StructColor`)))
  (set `self.EnumColor` newColor)
  (for (_array_element _array_index) (select `/Game/MyGame/Data/EnumColor` (`self.EnumColor`) :`NewEnumerator0` _mat_blue :`NewEnumerator1` _mat_red :`NewEnumerator2` _mat_yellow :`NewEnumerator3` _mat_green :`NewEnumerator4` _mat_none)
    (`PrimitiveComponent.SetMaterial` (`self.PlateformeMesh`) _array_index _array_element)
    (`self.NewEventDispatcher_0`)))

(fn `ResetColor`)

(fn `SetChildActorPosition`
  (bind _childactor (`self.childActor`))
  (bind (_returnvalue_roll _returnvalue_pitch _returnvalue_yaw) (`KismetMathLibrary.BreakRotator` (`SceneComponent.K2_GetComponentRotation` (`self.PlateformeMesh`))))
  (bind (_returnvalue_x _returnvalue_y _returnvalue_z) (`KismetMathLibrary.BreakVector` (+ (`KismetMathLibrary.MakeVector` _returnvalue_roll _returnvalue_pitch _returnvalue_yaw) (`self.childActorRotation`))))
  (`/Engine/EditorBlueprintResources/StandardMacros.IsValid` _childactor
    (:`Is Valid`
      (bind _asbp_color_detector (cast `/Game/MyGame/Blueprint/BP_ColorDetector` _childactor)
        (:`then`
          (set `/Game/MyGame/Blueprint/BP_ColorDetector.parentPlatform` self _asbp_color_detector))
        (:`CastFailed`
          _))
      (`self.K2_SetActorLocation` (`self.childActor`) (+ (`SceneComponent.K2_GetComponentLocation` (`self.PlateformeMesh`)) (`self.childActorOffset`)) false false)
      (`self.K2_SetActorRotation` (`self.childActor`) (`KismetMathLibrary.MakeRotator` _returnvalue_x _returnvalue_y _returnvalue_z) false))))

(fn `UserConstructionScript`
  (bind (_mat_none _mat_blue _mat_green _mat_yellow _mat_red) (break `/Game/MyGame/Data/StructColorText` (`self.StructColor`)))
  (for (_array_element _array_index) (select `/Game/MyGame/Data/EnumColor` (`self.EnumColor`) :`NewEnumerator0` _mat_blue :`NewEnumerator1` _mat_red :`NewEnumerator2` _mat_yellow :`NewEnumerator3` _mat_green :`NewEnumerator4` _mat_none)
    (`PrimitiveComponent.SetMaterial` (`self.PlateformeMesh`) _array_index _array_element))
  (`self.SetChildActorPosition`))