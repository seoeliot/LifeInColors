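; BP_ToolTip is a trigger actor that shows an on-screen tooltip while the first-person player is inside its Box.
; On begin overlap with BP_FirstPerson, it creates a WB_Tooltip from its TipID, adds it to the viewport and stores it.
; End overlap removes the stored widget from its parent.
; A DisplayOnce flag, paired with WasDisplayed, can limit the tooltip to the first entry.
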(event `self.Box.OnComponentBeginOverlap`
  (params (OverlappedComponent :type "PrimitiveComponent Object Reference") (OtherActor :type "Actor Object Reference") (OtherComp :type "PrimitiveComponent Object Reference") (OtherBodyIndex :type Integer) (bFromSweep :type Boolean) (SweepResult :type "HitResult Structure (by ref)"))
  (if (`self.displayOnce`)
    (if (not (`self.wasDisplayed`))
      (cast `/Game/MyGame/Joueur/Character/BP_FirstPerson` OtherActor :!label _label)
      (bind _returnvalue (`|CreateWidget` "/Game/MyGame/Tooltips/WB_Tooltip.WB_Tooltip_C" null (`self.Tip ID`)))
      (`UserWidget.AddToViewport` _returnvalue 0)
      (set `self.Widget` _returnvalue)
      (set `self.wasDisplayed` true))
    (else
      (goto _label))))

(event `self.Box.OnComponentEndOverlap`
  (params (OverlappedComponent :type "PrimitiveComponent Object Reference") (OtherActor :type "Actor Object Reference") (OtherComp :type "PrimitiveComponent Object Reference") (OtherBodyIndex :type Integer))
  (cast `/Game/MyGame/Joueur/Character/BP_FirstPerson` OtherActor)
  (`Widget.RemoveFromParent` (`self.Widget`)))

(fn `UserConstructionScript`)