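; In-game game mode that sets up the main HUD and plays timed dialogue sequences on screen.
; BeginPlay adds HUD_Main to the viewport and enables click and mouse-over events on the player controller.
; EventDialogue stores the lines, creates a WB_Dialogue widget and starts DialogueSuivant, which re-schedules itself by timer, scaling each delay with text length above a minimum.
; The widget is removed after the last line; the line index is never reset here.
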(event `EventDialogue`
  (params (Dialogue :type "Array of /Game/MyGame/Blueprint/Dialogue/S_LigneDeDialogue Structure"))
  ;[1 1 1] Dialogue
  (set `self.Dialogue` Dialogue)
  (bind _returnvalue (`|CreateWidget` "/Game/MyGame/UI_HUD/WB_Dialogue.WB_Dialogue_C"))
  (bind _output_get (set `self.DialogueWidget` _returnvalue))
  (`UserWidget.AddToViewport` _output_get 0)
  (`self.DialogueSuivant`))

(event `self.ReceiveBeginPlay`
  (bind _returnvalue (`GameplayStatics.GetPlayerController` 0))
  ;[0.3932 0.4388 1] Initialisation
  ;;[1 1 1] Main widget
  (bind _returnvalue_2 (`|CreateWidget` "/Game/MyGame/UI_HUD/HUD_Main.HUD_Main_C"))
  (`UserWidget.AddToViewport` _returnvalue_2 0)
  (set `PlayerController.bEnableMouseOverEvents` true _returnvalue)
  (set `PlayerController.bEnableClickEvents` true _returnvalue))

(fn `DialogueSuivant`
  (bind _dureedialogueminimum (`self.DureeDialogueMinimum`))
  (bind _output (`|GetArrayItem` (`self.Dialogue`) (`self.LigneDialogueCourante`)))
  (bind _returnvalue (* (`self.DureeDialogue`) (`KismetStringLibrary.Len` (`KismetTextLibrary.Conv_TextToString` (`.Lignededialogue_4_3B5F47EE4E9E86E649579CBE3DDB6D91` (break `/Game/MyGame/Blueprint/Dialogue/S_LigneDeDialogue` _output))))))
  (if (>= (`self.LigneDialogueCourante`) (`KismetArrayLibrary.Array_Length` (`self.Dialogue`)))
    (`Widget.RemoveFromParent` (`self.DialogueWidget`))
    (else
      (`/Game/MyGame/UI_HUD/WB_Dialogue.ChangerDialogue` (`self.DialogueWidget`) _output)
      (`KismetSystemLibrary.K2_SetTimer` null "DialogueSuivant" (`KismetMathLibrary.SelectFloat` _dureedialogueminimum _returnvalue (> _dureedialogueminimum _returnvalue)))
      (`/Engine/EditorBlueprintResources/StandardMacros.IncrementInt` (`self.LigneDialogueCourante`)))))

(fn `UserConstructionScript`)