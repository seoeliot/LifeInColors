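; GM_SAVED, apparently a game mode, sets up the main HUD and handles respawning of the first-person player character.
; BeginPlay creates the HUD widget, enables mouse click and hover events, and binds Mort to the character's OnDestroyed.
; After a delay, Mort spawns a replacement at SpawnTransform, possesses it, switches the view target, then calls Respawn to rebind the destruction event.
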(event `self.ReceiveBeginPlay`
  (bind _returnvalue (`GameplayStatics.GetPlayerController` 0))
  (`|ExecutionSequence`
    (:`then_0`
      (bind _returnvalue_2 (`|CreateWidget` "/Game/MyGame/UI_HUD/HUD_Main.HUD_Main_C"))
      (`UserWidget.AddToViewport` _returnvalue_2 0)
      (set `PlayerController.bEnableMouseOverEvents` true _returnvalue)
      (set `PlayerController.bEnableClickEvents` true _returnvalue))
    (:`then_1`
      (bind _asbp_first_person (cast `/Game/MyGame/Blueprint/BP_FirstPerson/BP_FirstPerson` (`GameplayStatics.GetPlayerCharacter` 0) :!label _label))
      (add `self.OnDestroyed` _asbp_first_person (delegate `Mort`)))))

(event `Respawn`
  (goto _label))

(event `Mort` :!signature `self.OnDestroyed`
  (params (DestroyedActor :type "Actor Object Reference"))
  (`KismetSystemLibrary.Delay` 2.0)
  (bind _returnvalue (`|SpawnActorFromClass` "/Game/MyGame/Blueprint/BP_FirstPerson/BP_FirstPerson.BP_FirstPerson_C" (`self.SpawnTransform`) "Undefined" "OverrideRootScale" null null))
  (`KismetSystemLibrary.Delay` 0.1)
  (`Controller.Possess` (`GameplayStatics.GetPlayerController` 0) _returnvalue)
  (`PlayerController.SetViewTargetWithBlend` (`GameplayStatics.GetPlayerController` 0) (`GameplayStatics.GetPlayerCharacter` 0) 0.0 "VTBlend_Linear" 0.0 false)
  (`self.Respawn`))

(fn `UserConstructionScript`)