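; Mine zone for Level01 that explodes when an actor tagged TriggerMine overlaps its ZoneBoom component.
; Any such actor is destroyed, Mort is set to true on GI_Main, and the MineBoom sound and particle system play.
; For actors without the Joueur (player) tag, it also changes the Zone material and sets BoomBoom, blocking further triggers.
; The player branch leaves BoomBoom unset, so the mine stays armed.
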(event `self.ZoneBoom.OnComponentBeginOverlap`
  (params (OverlappedComponent :type "PrimitiveComponent Object Reference") (OtherActor :type "Actor Object Reference") (OtherComp :type "PrimitiveComponent Object Reference") (OtherBodyIndex :type Integer) (bFromSweep :type Boolean) (SweepResult :type "HitResult Structure (by ref)"))
  (if (`self.BoomBoom?`)
    _
    (elif (`self.ActorHasTag` OtherActor "TriggerMine")
      (if (`self.ActorHasTag` OtherActor "Joueur")
        (`self.K2_DestroyActor` OtherActor)
        (bind _asgi_main (cast `/Game/MyGame/Data/GameInstance/GI_Main` (`GameplayStatics.GetGameInstance`)))
        (set `/Game/MyGame/Data/GameInstance/GI_Main.Mort?` true _asgi_main)
        (`GameplayStatics.PlaySound2D` "/Game/MyGame/Sound/SoundEffect/MineBoom.MineBoom" 1.0 1.0 0.0 null null)
        (`ActorComponent.Activate` (`self.ParticleSystem`) false)
        (else
          (`self.K2_DestroyActor` OtherActor)
          (`PrimitiveComponent.SetMaterial` (`self.Zone`) 0 "/Game/UE5/StarterContent/Materials/M_Tech_Hex_Tile.M_Tech_Hex_Tile")
          (bind _asgi_main_2 (cast `/Game/MyGame/Data/GameInstance/GI_Main` (`GameplayStatics.GetGameInstance`)))
          (set `/Game/MyGame/Data/GameInstance/GI_Main.Mort?` true _asgi_main_2)
          (`GameplayStatics.PlaySound2D` "/Game/MyGame/Sound/SoundEffect/MineBoom.MineBoom" 1.0 1.0 0.0 null null)
          (`ActorComponent.Activate` (`self.ParticleSystem`) false)
          (set `self.BoomBoom?` true))))))

(fn `UserConstructionScript`)