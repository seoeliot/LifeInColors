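; BP_PlateformBoom is a Level01 actor, apparently an exploding platform, that blows up and removes itself when the first-person player touches it.
; The Box overlap event filters for BP_FirstPerson, then plays the MineBoom sound in 2D.
; It activates three explosion components in a short staggered sequence using delays, then destroys the actor.
; No damage or impulse is applied in this Blueprint.
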(event `self.Box.OnComponentBeginOverlap`
  (params (OverlappedComponent :type "PrimitiveComponent Object Reference") (OtherActor :type "Actor Object Reference") (OtherComp :type "PrimitiveComponent Object Reference") (OtherBodyIndex :type Integer) (bFromSweep :type Boolean) (SweepResult :type "HitResult Structure (by ref)"))
  (cast `/Game/MyGame/Joueur/Character/BP_FirstPerson` OtherActor)
  (`GameplayStatics.PlaySound2D` "/Game/MyGame/Sound/SoundEffect/MineBoom.MineBoom" 1.0 1.0 0.0 null null)
  (`ActorComponent.Activate` (`self.EXPLOSION`) false)
  (`KismetSystemLibrary.Delay` 0.1)
  (`ActorComponent.Activate` (`self.EXPLOSION1`) false)
  (`KismetSystemLibrary.Delay` 0.1)
  (`ActorComponent.Activate` (`self.EXPLOSION2`) false)
  (`KismetSystemLibrary.Delay` 0.2)
  (`self.K2_DestroyActor`))

(fn `UserConstructionScript`)