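; BP_HubFog tints the exponential height fog in the hub level according to game progression.
; On BeginPlay it picks a target color from GI_Main's ProgressionState and binds to that game instance's OnUnlockColor event, unbinding on EndPlay.
; Tick blends the fog inscattering color toward the target using DeltaSeconds as lerp alpha, giving an eased transition.
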(event `ChangeColor`
  (bind _asgi_main (cast `/Game/MyGame/Data/GameInstance/GI_Main` (`GameplayStatics.GetGameInstance`)))
  (set `self.NewColor` (select `/Game/MyGame/Data/GameInstance/ProgressionState` (`/Game/MyGame/Data/GameInstance/GI_Main.ProgressionState` _asgi_main) :`NewEnumerator0` (struct :`R` 1.0 :`A` 1.0) :`NewEnumerator6` (struct :`G` 1.0 :`A` 1.0) :`NewEnumerator1` (struct :`B` 1.0 :`A` 1.0) :`NewEnumerator2` (struct :`R` 1.0 :`G` 0.83201 :`A` 1.0) :`NewEnumerator3` (struct :`R` 1.0 :`G` 1.0 :`B` 1.0 :`A` 1.0) :`NewEnumerator4` (struct :`R` 1.0 :`G` 1.0 :`B` 1.0 :`A` 1.0) :!type "LinearColor Structure")))

(event `self.ReceiveBeginPlay`
  (bind _asgi_main (cast `/Game/MyGame/Data/GameInstance/GI_Main` (`GameplayStatics.GetGameInstance`)))
  (add `/Game/MyGame/Data/GameInstance/GI_Main.OnUnlockColor` _asgi_main (`|CreateDelegate` :!event `ChangeColor`))
  (`self.ChangeColor`))

(event `self.ReceiveEndPlay`
  (params (EndPlayReason :type "EEndPlayReason Enum" :default "Destroyed"))
  (bind _asgi_main (cast `/Game/MyGame/Data/GameInstance/GI_Main` (`GameplayStatics.GetGameInstance`)))
  (remove `/Game/MyGame/Data/GameInstance/GI_Main.OnUnlockColor` _asgi_main (`|CreateDelegate` :!event `ChangeColor`)))

(event `self.ReceiveTick`
  (params (DeltaSeconds :type "Float (single-precision)"))
  (`ExponentialHeightFogComponent.SetFogInscatteringColor` (`self.ExponentialHeightFog`) (`KismetMathLibrary.LinearColorLerp` (`ExponentialHeightFogComponent.FogInscatteringLuminance` (`self.ExponentialHeightFog`)) (`self.NewColor`) DeltaSeconds)))

(fn `UserConstructionScript`)