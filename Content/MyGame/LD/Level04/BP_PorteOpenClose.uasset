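; BP_PorteOpenClose is a Level04 door actor that swings open and closed continuously by itself, with no player trigger.
; From BeginPlay it runs an endless delay loop that switches between two RotatingMovement components, presumably set to opposite directions.
; Each cycle activates one component, pauses with both off, activates the other, then pauses again, all at equal fixed intervals.
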(event `self.ReceiveBeginPlay`
  (`KismetSystemLibrary.Delay` 2.0 :!label _label)
  (`ActorComponent.SetActive` (`self.RotatingMovement1`) true false)
  (`ActorComponent.SetActive` (`self.RotatingMovement`) false false)
  (`KismetSystemLibrary.Delay` 2.0)
  (`ActorComponent.SetActive` (`self.RotatingMovement1`) false false)
  (`ActorComponent.SetActive` (`self.RotatingMovement`) false false)
  (`KismetSystemLibrary.Delay` 2.0)
  (`ActorComponent.SetActive` (`self.RotatingMovement1`) false false)
  (`ActorComponent.SetActive` (`self.RotatingMovement`) true false)
  (`KismetSystemLibrary.Delay` 2.0)
  (`ActorComponent.SetActive` (`self.RotatingMovement1`) false false)
  (`ActorComponent.SetActive` (`self.RotatingMovement`) false false)
  (goto _label))

(fn `UserConstructionScript`)