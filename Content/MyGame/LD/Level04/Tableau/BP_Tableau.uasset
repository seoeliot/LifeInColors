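; BP_Tableau is a painting prop for Level04 that shows an artwork with a title and author label.
; It applies the Tableau material to the first material slot of its Cube and writes the TitreAuteur text to its TextRender.
; The same two calls run in both the Construction Script and BeginPlay, so the result also previews in the editor.
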(event `self.ReceiveBeginPlay`
  (`PrimitiveComponent.SetMaterial` (`self.Cube`) 0 (`self.Tableau`))
  (`TextRenderComponent.K2_SetText` (`self.TextRender`) (`self.TitreAuteur`)))

(fn `UserConstructionScript`
  (`PrimitiveComponent.SetMaterial` (`self.Cube`) 0 (`self.Tableau`))
  (`TextRenderComponent.K2_SetText` (`self.TextRender`) (`self.TitreAuteur`)))