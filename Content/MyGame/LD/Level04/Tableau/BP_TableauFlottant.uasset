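; BP_TableauFlottant is a floating painting (tableau) actor for Level04 that spins continuously at a random speed.
; On BeginPlay it applies the Tableau material to its Cube, waits briefly, then sets the RotatingMovement component's rotation rate.
; A coin flip picks positive or negative rotation for all three axes together, with each axis speed randomized independently.
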(event `self.ReceiveBeginPlay`
  (bind _returnvalue (* (`KismetMathLibrary.RandomFloat`) 30.0))
  (bind _returnvalue_2 (* (`KismetMathLibrary.RandomFloat`) 30.0))
  (bind _returnvalue_3 (* (`KismetMathLibrary.RandomFloat`) 30.0))
  (`PrimitiveComponent.SetMaterial` (`self.Cube`) 0 (`self.Tableau`))
  (`KismetSystemLibrary.Delay` 0.01)
  (if (`KismetMathLibrary.RandomBool`)
    (set `RotatingMovementComponent.RotationRate` (`KismetMathLibrary.MakeRotator` _returnvalue_2 _returnvalue_3 _returnvalue) (`self.RotatingMovement`))
    (else
      (set `RotatingMovementComponent.RotationRate` (`KismetMathLibrary.MakeRotator` (* _returnvalue_2 -1.0) (* _returnvalue_3 -1.0) (* _returnvalue -1.0)) (`self.RotatingMovement`)))))

(fn `UserConstructionScript`)