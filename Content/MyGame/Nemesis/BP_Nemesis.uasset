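; BP_Nemesis is an enemy character that chases the player and destroys them on reaching them.
; On BeginPlay it sets its walk speed from SpeedNemesis, then uses AIMoveTo to target the first player's character.
; A failed move restarts the chase through the GoToPlayer event, while a successful one prints a debug message and destroys the player character.
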(event `self.ReceiveBeginPlay`
  (set `CharacterMovementComponent.MaxWalkSpeed` (`self.SpeedNemesis`) (`self.CharacterMovement`))
  (`self.GoToPlayer`))

(event `GoToPlayer`
  (bind _returnvalue (`GameplayStatics.GetPlayerCharacter` 0))
  (`|AIMoveTo` self (0.0 0.0 0.0) _returnvalue
    (:`OnSuccess`
      (`KismetSystemLibrary.PrintString` "JE T'AI EU JE SUIS TOI EN FAIT")
      (`self.K2_DestroyActor` _returnvalue))
    (:`OnFail`
      (`self.GoToPlayer`))))

(fn `UserConstructionScript`)