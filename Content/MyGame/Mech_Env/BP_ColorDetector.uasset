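; Color detector that fires a begin trigger when a visible paintable cube or activable conveyor of its color is inside its capsule.
; Each Tick, it filters capsule overlaps with a line-of-sight sphere trace and color match, calling end trigger whenever none qualifies.
; A forward line trace resizes the beam decal to the first blocking hit, while the Construction Script colors mesh and decal.
; Mobile platforms are sight-checked but never activate it.
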(event `self.ReceiveTick`
  (params (DeltaSeconds :type "Float (single-precision)"))
  (bind _decal (`self.Decal`))
  (bind _returnvalue (`SceneComponent.K2_GetComponentLocation` (`self.SphereTraceStartPoint`)))
  (bind (_relativelocation_x _relativelocation_y) (`KismetMathLibrary.BreakVector` (`SceneComponent.RelativeLocation` _decal)))
  (`|ExecutionSequence`
    (:`then_0`
      (bind _outactors (`GameplayStatics.GetAllActorsWithTag` (`self.DecalNoBlockTag`)))
      (bind _outhit (`KismetSystemLibrary.LineTraceSingle` _returnvalue (+ _returnvalue (* (`SceneComponent.GetForwardVector` (`self.Arrow`)) (`self.Range`))) "TraceTypeQuery1" false _outactors))
      (bind _returnvalue_2 (/ (`.Distance` (`GameplayStatics.BreakHitResult` _outhit)) 1.9))
      (`SceneComponent.SetRelativeScale3D` _decal (`KismetMathLibrary.MakeVector` _returnvalue_2 150.0 150.0))
      (`SceneComponent.K2_SetRelativeLocation` _decal (`KismetMathLibrary.MakeVector` _relativelocation_x _relativelocation_y (+ _returnvalue_2 100.0)) false false))
    (:`then_1`
      (set `self.bFoundColor` false)
      (for _array_element (`PrimitiveComponent.GetOverlappingActors` (`self.Capsule`) null)
        (bind _asbp_paintable_cube (cast `/Game/MyGame/Mech_Color/Paintable/Cube/BP_PaintableCube` _array_element)
          (:`then`
            (bind _bobjecthit (`self.Check Object in Sight` _asbp_paintable_cube))
            (if (and _bobjecthit (`|EnumEquality` (`/Game/MyGame/Mech_Color/Paintable/Cube/BP_PaintableCube.Color` _asbp_paintable_cube) (`self.Color`)))
              (set `self.bFoundColor` true :!label _label)
              (if (not (`self.bIsActivated`))
                (set `self.bIsActivated` true)
                (`self.BeginTrigger`)
                (`KismetSystemLibrary.PrintString` "Hit color !" true true (struct :`G` 0.66 :`B` 1.0 :`A` 1.0) 1.0)
                (`GameplayStatics.PlaySound2D` "/Game/MyGame/Sound/SoundEffect/Bonus.Bonus" 1.0 1.0 0.0 null null))))
          (:`CastFailed`
            (bind _asbp_plateforme_mobile (cast `/Game/MyGame/Mech_Color/Paintable/Plateforme/BP_PlateformeMobile` _array_element)
              (:`then`
                (`self.Check Object in Sight` _asbp_plateforme_mobile))
              (:`CastFailed`
                (bind _asbp_activable_conveyor (cast `/Game/MyGame/Mech_Color/Paintable/Tapis/BP_ActivableConveyor` _array_element))
                (bind _bobjecthit_2 (`self.Check Object in Sight` _asbp_activable_conveyor))
                (if (and _bobjecthit_2 (`|EnumEquality` (`/Game/MyGame/Mech_Color/Paintable/Tapis/BP_ActivableConveyor.Color` _asbp_activable_conveyor) (`self.Color`)))
                  (goto _label)))))))
      (if (not (`self.bFoundColor`))
        (set `self.bIsActivated` false)
        (`self.EndTrigger`)))))

(fn `Check Object in Sight`
  (params (other :type "Actor Object Reference"))
  (returns (bObjectHit :type Boolean))
  (locals (localOther :type "Actor Object Reference"))
  (bind _output_get (set `local.localOther` other))
  (bind _outactors (`GameplayStatics.GetAllActorsWithTag` (`self.DetectionNoBlockTag`)))
  (`KismetArrayLibrary.Array_Add` _outactors (`self.parentPlatform`))
  (bind _outhit (`KismetSystemLibrary.SphereTraceSingle` (`SceneComponent.K2_GetComponentLocation` (`self.SphereTraceStartPoint`)) (`SceneComponent.K2_GetComponentLocation` (`Actor.RootComponent` _output_get)) 50.0 "TraceTypeQuery1" false _outactors))
  (return (== (`.HitActor` (`GameplayStatics.BreakHitResult` _outhit)) (`local.localOther`))))

(fn `UserConstructionScript`
  (bind _returnvalue (/ 1000.0 1.9))
  (bind _decal (`self.Decal`))
  (bind (_relativelocation_x _relativelocation_y) (`KismetMathLibrary.BreakVector` (`SceneComponent.RelativeLocation` _decal)))
  (`PrimitiveComponent.SetMaterial` (`self.StaticMesh`) 0 (select `/Game/MyGame/Data/Enum_Struct/EnumColor` (`self.Color`) :`NewEnumerator0` "/Game/MyGame/Mech_Color/Materials/Mat_Blue.Mat_Blue" :`NewEnumerator1` "/Game/MyGame/Mech_Color/Materials/Mat_Red.Mat_Red" :`NewEnumerator2` "/Game/MyGame/Mech_Color/Materials/Mat_Yellow.Mat_Yellow" :`NewEnumerator4` "/Game/UE5/FPWeapon/Materials/BaseMaterial.BaseMaterial" :!type "MaterialInterface Object Reference"))
  (`DecalComponent.SetDecalMaterial` (`self.Decal`) (select `/Game/MyGame/Data/Enum_Struct/EnumColor` (`self.Color`) :`NewEnumerator0` "/Game/MyGame/Mech_Color/Materials/Mat_DecalBlue.Mat_DecalBlue" :`NewEnumerator1` "/Game/MyGame/Mech_Color/Materials/Mat_DecalRed.Mat_DecalRed" :`NewEnumerator2` "/Game/MyGame/Mech_Color/Materials/Mat_DecalYellow.Mat_DecalYellow" :`NewEnumerator4` "/Game/UE5/FPWeapon/Materials/BaseMaterial.BaseMaterial" :!type "MaterialInterface Object Reference"))
  (`SceneComponent.SetRelativeScale3D` _decal (`KismetMathLibrary.MakeVector` _returnvalue 150.0 150.0))
  (`SceneComponent.K2_SetRelativeLocation` _decal (`KismetMathLibrary.MakeVector` _relativelocation_x _relativelocation_y (+ _returnvalue 100.0)) false false))