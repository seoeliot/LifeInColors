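; BP_Connection is an environment mechanic actor that visually links a Trigger to an Activable with a colored effect.
; The construction script snaps the spline's first and last points to both actors' offset locations and sets the color on NGRConnection.
; Tick polls the trigger's activated state, using a resettable DoOnce to activate the effect once per activation and deactivating it otherwise.
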(event `self.ReceiveTick`
  (params (DeltaSeconds :type "Float (single-precision)"))
  (bind _ngr_connection (`self.NGR_Connection`))
  (`|ExecutionSequence`
    (:`then_0`
      (if (`/Game/MyGame/Mech_Env/BP_Trigger.bIsActivated` (`self.Trigger`))
        (`/Engine/EditorBlueprintResources/StandardMacros.DoOnce` false :!label _label
          (:`Completed`
            (`ActorComponent.Activate` _ngr_connection true)))
        (else
          (`ActorComponent.Deactivate` _ngr_connection)
          (goto _label :!via `Reset`))))))

(fn `UserConstructionScript`
  (bind _spline (`self.Spline`))
  (bind _trigger (`self.Trigger`))
  (bind _activable (`self.Activable`))
  (`|ExecutionSequence`
    (:`then_0`
      (`/Engine/EditorBlueprintResources/StandardMacros.IsValid` _trigger
        (:`Is Valid`
          (`SplineComponent.SetLocationAtSplinePoint` (`self.Spline`) 0 (+ (`self.K2_GetActorLocation` _trigger) (`/Game/MyGame/Mech_Env/BP_Trigger.ConnectionOffset` _trigger)) "World" true))
        (:`Is Not Valid`
          _))
      (`/Engine/EditorBlueprintResources/StandardMacros.IsValid` _activable
        (:`Is Valid`
          (`SplineComponent.SetLocationAtSplinePoint` _spline (- (`SplineComponent.GetNumberOfSplinePoints` _spline) 1) (+ (`self.K2_GetActorLocation` _activable) (`/Game/MyGame/Mech_Env/BP_Activable.ConnectionStartOffset` _activable)) "World" true))))
    (:`then_1`
      (`FXSystemComponent.SetColorParameter` (`self.NGR_Connection`) "Color" (`self.Color`)))))