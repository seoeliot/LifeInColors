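; BP_ActivableDoor is a door that opens when its Action event receives a trigger count equal to TriggerCount.
; BeginPlay caches the actor's starting location and calls BeginFunction, which is not defined in this graph.
; Action prints a debug string, then opens the door by moving it to a fixed far-off relative location, or otherwise sets it to the cached start, without sweep or animation.
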(event `self.ReceiveBeginPlay`
  (set `self.LocationStart` (`self.K2_GetActorLocation`))
  (`self.BeginFunction`))

(event `self.Action`
  (params (currentTrigger :type Integer))
  (`KismetSystemLibrary.PrintString` "Hello")
  (if (== currentTrigger (`self.triggerCount`))
    (`self.K2_SetActorRelativeLocation` (0.0 0.0 10000.0))
    (else
      (`self.K2_SetActorRelativeLocation` (`self.LocationStart`)))))

(fn `UserConstructionScript`)