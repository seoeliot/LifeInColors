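; BP_Vinyle is a collectible vinyl record that registers itself when the player interacts with it.
; On interact it adds its Numero to the VinylesList in the GI_Main game instance, shows a WB_NotifJournal notification, calls DestroyNotif on it and destroys itself.
; DisplayInteractHUD and HideInteractHUD toggle the visibility of its Widget component as the interaction prompt.
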(event `/Game/MyGame/Mech_Env/BPI_Interractible.OnInteract`
  (params (`Player Ref` :type "/Game/MyGame/Joueur/Character/BP_FirstPerson Object Reference"))
  (bind _asgi_main (cast `/Game/MyGame/Data/GameInstance/GI_Main` (`GameplayStatics.GetGameInstance`)))
  (`KismetArrayLibrary.Array_Add` (`/Game/MyGame/Data/GameInstance/GI_Main.VinylesList` _asgi_main) (`self.Numero `))
  (bind _returnvalue (`|CreateWidget` "/Game/MyGame/UI_HUD/Journal/WB_NotifJournal.WB_NotifJournal_C"))
  (`UserWidget.AddToViewport` _returnvalue 0)
  (`/Game/MyGame/UI_HUD/Journal/WB_NotifJournal.DestroyNotif` _returnvalue)
  (`self.K2_DestroyActor`))

(event `/Game/MyGame/Mech_Env/BPI_Interractible.DisplayInteractHUD`
  (`SceneComponent.SetVisibility` (`self.Widget`) true false))

(event `/Game/MyGame/Mech_Env/BPI_Interractible.HideInteractHUD`
  (`SceneComponent.SetVisibility` (`self.Widget`) false false))

(fn `UserConstructionScript`)