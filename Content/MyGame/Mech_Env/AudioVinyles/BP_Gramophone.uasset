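; BP_Gramophone is an interactable gramophone actor that opens the gramophone UI when the player uses it.
; On interact it pauses the game, shows the mouse cursor, then creates a WB_Gramophone widget and adds it to the viewport.
; Display and hide HUD events toggle the visibility of its Widget component as an interaction prompt.
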(event `/Game/MyGame/Mech_Env/BPI_Interractible.OnInteract`
  (params (`Player Ref` :type "/Game/MyGame/Joueur/Character/BP_FirstPerson Object Reference"))
  (`GameplayStatics.SetGamePaused` true)
  (set `PlayerController.bShowMouseCursor` true (`GameplayStatics.GetPlayerController` 0))
  (bind _returnvalue (`|CreateWidget` "/Game/MyGame/Mech_Env/AudioVinyles/WB_Gramophone.WB_Gramophone_C"))
  (`UserWidget.AddToViewport` _returnvalue 0))

(event `/Game/MyGame/Mech_Env/BPI_Interractible.DisplayInteractHUD`
  (`SceneComponent.SetVisibility` (`self.Widget`) true false))

(event `/Game/MyGame/Mech_Env/BPI_Interractible.HideInteractHUD`
  (`SceneComponent.SetVisibility` (`self.Widget`) false false))

(fn `UserConstructionScript`)