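; BP_Soldat is a soldier actor that holds a rifle aiming idle animation until a color change triggers its one-time scripted exit.
; The first ChangeColor call, guarded by a DoOne flag, creates and plays a level sequence selected by color, with only Red having one assigned.
; It then sends its Dialogue to GM_InGame and destroys itself after a delay based on the sequence's end time.
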(event `self.ReceiveBeginPlay`
  (`SkeletalMeshComponent.SetAnimation` (`self.Mesh`) "/Game/MyGame/Mech_Env/AudioVinyles/Fragment/FBX/Soldat/Rifle_Aiming_Idle_Anim_mixamo_com.Rifle_Aiming_Idle_Anim_mixamo_com"))

(event `/Game/MyGame/Mech_Color/Paintable/BPI_Paintable.ChangeColor`
  (params (newColor :type "/Game/MyGame/Data/Enum_Struct/EnumColor Enum" :default "NewEnumerator0"))
  (if (not (`self.DoOne`))
    (set `self.DoOne` true)
    (bind _outactor (`LevelSequencePlayer.CreateLevelSequencePlayer` (select `/Game/MyGame/Data/Enum_Struct/EnumColor` newColor :`NewEnumerator1` "/Game/MyGame/Mech_Env/AudioVinyles/Fragment/LevelSequence.LevelSequence" :!type "LevelSequence Object Reference")))
    (bind _sequenceplayer (`LevelSequenceActor.SequencePlayer` _outactor))
    (`MovieSceneSequencePlayer.Play` _sequenceplayer)
    (bind _asgm_in_game (cast `/Game/MyGame/Data/GameInstance/GM_InGame` (`GameplayStatics.GetGameMode`)))
    (`/Game/MyGame/Data/GameInstance/GM_InGame.EventDialogue` _asgm_in_game (`self.Dialogue`))
    (`KismetSystemLibrary.Delay` (`TimeManagementBlueprintLibrary.Conv_QualifiedFrameTimeToSeconds` (`MovieSceneSequencePlayer.GetEndTime` _sequenceplayer)))
    (`self.K2_DestroyActor`)))

(fn `UserConstructionScript`)