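; BP_P_Fragment is a trigger that plays a Level Sequence when the first-person player enters its box, then removes a soldier.
; On overlap it creates a sequence player, plays it and delays for the sequence's end time in seconds.
; It then destroys the first BP_Soldat found in the level.
; The overlap has no once-only guard, and an unfinished actor-search loop is never run.
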(event `self.Box.OnComponentBeginOverlap`
  (params (OverlappedComponent :type "PrimitiveComponent Object Reference") (OtherActor :type "Actor Object Reference") (OtherComp :type "PrimitiveComponent Object Reference") (OtherBodyIndex :type Integer) (bFromSweep :type Boolean) (SweepResult :type "HitResult Structure (by ref)"))
  (cast `/Game/MyGame/Joueur/Character/BP_FirstPerson` OtherActor)
  (bind _outactor (`LevelSequencePlayer.CreateLevelSequencePlayer` "/Game/MyGame/Mech_Env/AudioVinyles/Fragment/LevelSequence.LevelSequence"))
  (bind _sequenceplayer (`LevelSequenceActor.SequencePlayer` _outactor))
  (`MovieSceneSequencePlayer.Play` _sequenceplayer)
  (`KismetSystemLibrary.Delay` (`TimeManagementBlueprintLibrary.Conv_QualifiedFrameTimeToSeconds` (`MovieSceneSequencePlayer.GetEndTime` _sequenceplayer)))
  (bind _outactors (`GameplayStatics.GetAllActorsOfClass` "/Game/MyGame/Mech_Env/AudioVinyles/Fragment/FBX/BP_Soldat.BP_Soldat_C"))
  (`self.K2_DestroyActor` (`|GetArrayItem` _outactors)))

(fn `UserConstructionScript`)