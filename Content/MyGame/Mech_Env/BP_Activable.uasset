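; Base actor for environment mechanisms driven by a set of trigger actors, with an empty Action event as the hook for behavior.
; On BeginPlay it binds to each trigger's begin and end events and stores the trigger count.
; UpdateTrigger counts the currently activated triggers and passes that total to Action.
; The construction script aims and stretches a single arrow toward linked triggers, so only the last one processed is shown.
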(event `self.ReceiveBeginPlay`
  (`self.BeginFunction`))

(event `UpdateTrigger`
  (bind _currenttrigger (`self.CalculateCurrentEnergy`))
  (`self.Action` _currenttrigger))

(event `Action`
  (params (currentTrigger :type Integer)))

(fn `BeginFunction`
  (bind _result (`BlueprintSetLibrary.Set_ToArray` (`self.TriggerSet`)))
  (for _array_element _result
    (add `/Game/MyGame/Mech_Env/BP_Trigger.BeginTrigger` _array_element (`|CreateDelegate` :!event `UpdateTrigger`))
    (add `/Game/MyGame/Mech_Env/BP_Trigger.EndTrigger` _array_element (`|CreateDelegate` :!event `UpdateTrigger`)))
  (set `self.triggerCount` (`BlueprintSetLibrary.Set_Length` (`self.TriggerSet`))))

(fn `CalculateCurrentEnergy`
  (returns (currentTrigger :type Integer))
  (set `self.currentTrigger` 0)
  (bind _result (`BlueprintSetLibrary.Set_ToArray` (`self.TriggerSet`)))
  (for _array_element _result
    (if (`/Game/MyGame/Mech_Env/BP_Trigger.bIsActivated` _array_element)
      (`/Engine/EditorBlueprintResources/StandardMacros.IncrementInt` (`self.currentTrigger`)
        (:`  `
          (`KismetSystemLibrary.PrintString` (`KismetStringLibrary.Conv_IntToString` (`self.currentTrigger`)) true true (struct :`G` 0.66 :`B` 1.0 :`A` 1.0) 0.0)))))
  (return (`self.currentTrigger`)))

(fn `ConstructionFunction`
  (bind _returnvalue (`self.K2_GetActorLocation`))
  (bind _arrow (`self.Arrow`))
  (`SceneComponent.SetWorldScale3D` (`self.Arrow`) (1.0 1.0 1.0))
  (bind _result (`BlueprintSetLibrary.Set_ToArray` (`self.TriggerSet`)))
  (for _array_element _result
    (`/Engine/EditorBlueprintResources/StandardMacros.IsValid` _array_element
      (:`Is Valid`
        (`SceneComponent.SetVisibility` _arrow true false)
        (bind _returnvalue_2 (`self.K2_GetActorLocation` _array_element))
        (`SceneComponent.K2_SetWorldRotation` _arrow (`KismetMathLibrary.FindLookAtRotation` _returnvalue _returnvalue_2) false false)
        (set `ArrowComponent.ArrowLength` (`KismetMathLibrary.Vector_Distance` _returnvalue _returnvalue_2) _arrow))
      (:`Is Not Valid`
        (`SceneComponent.SetVisibility` _arrow false false)))))

(fn `UserConstructionScript`
  (`self.ConstructionFunction`))