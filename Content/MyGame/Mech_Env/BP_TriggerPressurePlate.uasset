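; Pressure plate trigger that activates while an actor tagged TriggerPressurePlate rests inside its box.
; Tick polls the box's overlapping actors rather than using overlap events, and an IsActivated flag limits responses to state changes.
; On press it calls BeginTrigger, lowers the cylinder and plays a click sound.
; Once no tagged actor remains, it calls EndTrigger and raises the cylinder silently.
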(event `self.ReceiveTick`
  (params (DeltaSeconds :type "Float (single-precision)"))
  (set `self.bFoundPressure` false)
  (for _array_element (`PrimitiveComponent.GetOverlappingActors` (`self.Box`) null)
    (if (`self.ActorHasTag` _array_element "TriggerPressurePlate")
      (set `self.bFoundPressure` true)
      (if (not (`self.bIsActivated`))
        (set `self.bIsActivated` true)
        (`self.BeginTrigger`)
        (`SceneComponent.K2_SetRelativeLocation` (`self.Cylinder`) (0.0 0.0 0.0) false false)
        (`GameplayStatics.PlaySoundAtLocation` "/Game/MyGame/Sound/SoundEffect/Button_Plate_Click__Minecraft_Sound__-_Sound_Effect_for_editing.Button_Plate_Click__Minecraft_Sound__-_Sound_Effect_for_editing" (`SceneComponent.K2_GetComponentLocation` (`self.Cylinder`)) (struct) 1.0 1.0 0.0 null null null null))))
  (if (`self.bFoundPressure`)
    _
    (elif (`self.bIsActivated`)
      (set `self.bIsActivated` false)
      (`self.EndTrigger`)
      (`SceneComponent.K2_SetRelativeLocation` (`self.Cylinder`) (0.0 0.0 5.0) false false))))

(fn `UserConstructionScript`)