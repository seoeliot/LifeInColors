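; Data Blueprint that tracks which BP_TableauTP paintings are painted blue, red or yellow, by their NameRef.
; UpdateV2 clears a painting's previous slot through WasColored, then files it under its new color or drops it from TPAll for None.
; Each color array works as a two-slot, newest-first queue.
; When both slots are full, SuprTableau finds the oldest painting's actor and resets its color to None.
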(event `self.ReceiveBeginPlay`)

(fn `AddTableau`
  (params (TargetArray :type "Array of String (by ref)"))
  (locals (RefTableau :type "Array of String"))
  (if (not (`KismetStringLibrary.EqualEqual_StrStr` (`|GetArrayItem` TargetArray)))
    (if (not (`KismetStringLibrary.EqualEqual_StrStr` (`|GetArrayItem` TargetArray 1)))
      (`self.SuprTableau` TargetArray))
    (`KismetArrayLibrary.Array_Set` TargetArray 1 (`|GetArrayItem` TargetArray)))
  (`KismetArrayLibrary.Array_Set` TargetArray 0 (`/Game/MyGame/Mech_Color/Paintable/TableauTP/BP_TableauTP.NameRef` (`self.Tableau`))))

(fn `Find Array`
  (params (ItemToFind :type "String (by ref)"))
  (returns (Array :type "Array of String"))
  (if (`KismetArrayLibrary.Array_Contains` (`self.TP_Bleu`) ItemToFind)
    (return (`self.TP_Bleu`))
    (elif (`KismetArrayLibrary.Array_Contains` (`self.TP_Jaune`) ItemToFind)
      (return (`self.TP_Jaune`))
      (elif (`KismetArrayLibrary.Array_Contains` (`self.TP_Rouge`) ItemToFind)
        (return (`self.TP_Rouge`))))))

(fn `FirstIndex?`
  (params (Array :type "Array of String") (Index :type String))
  (returns (`IsFirstIndex?` :type Boolean))
  (return (`KismetStringLibrary.EqualEqual_StrStr` Index (`|GetArrayItem` Array))))

(fn `SuprTableau`
  (params (Array :type "Array of String"))
  (bind _outactors (`GameplayStatics.GetAllActorsOfClass` "/Game/MyGame/Mech_Color/Paintable/TableauTP/BP_TableauTP.BP_TableauTP_C"))
  (for _array_element _outactors
    (if (`KismetStringLibrary.EqualEqual_StrStr` (`/Game/MyGame/Mech_Color/Paintable/TableauTP/BP_TableauTP.NameRef` _array_element) (`|GetArrayItem` Array 1))
      (`/Game/MyGame/Mech_Color/Paintable/TableauTP/BP_TableauTP.ChangementDeCouleur` _array_element "NewEnumerator4")
      (break))))

(fn `UpdateV2`
  (params (NouvelleCouleur :type "/Game/MyGame/Data/Enum_Struct/EnumColor Enum" :default "NewEnumerator0") (Tableau :type "/Game/MyGame/Mech_Color/Paintable/TableauTP/BP_TableauTP Object Reference"))
  (set `self.Tableau` Tableau)
  (set `self.Nouvelle Couleur` NouvelleCouleur)
  ;[1 1 1] Verifie si le tableau avait déjà une couleur
  (`self.WasColored?`)
  (switch `/Game/MyGame/Data/Enum_Struct/EnumColor` (`self.Nouvelle Couleur`)
    (:`NewEnumerator0`
      (`self.AddTableau` (`self.TP_Bleu`))
      (for _array_element (`self.TP_All`) :!label _label
        (`KismetSystemLibrary.PrintString` _array_element)))
    (:`NewEnumerator1`
      (`self.AddTableau` (`self.TP_Rouge`))
      (goto _label))
    (:`NewEnumerator2`
      (`self.AddTableau` (`self.TP_Jaune`))
      (goto _label))
    (:`NewEnumerator4`
      (`KismetArrayLibrary.Array_RemoveItem` (`self.TP_All`) (`/Game/MyGame/Mech_Color/Paintable/TableauTP/BP_TableauTP.NameRef` (`self.Tableau`))))))

(fn `UserConstructionScript`)

(fn `WasColored?`
  (locals (RefTableau :type "Array of String"))
  (bind _tp_all (`self.TP_All`))
  (bind _nameref (`/Game/MyGame/Mech_Color/Paintable/TableauTP/BP_TableauTP.NameRef` (`self.Tableau`)))
  (if (`KismetArrayLibrary.Array_Contains` _tp_all _nameref)
    (bind _array (`self.Find Array` _nameref))
    (bind _isfirstindex_ (`self.FirstIndex?` _array _nameref))
    ;[1 1 1] On enleve de la mémoire l'ancienne couleur du tableau
    (if _isfirstindex_
      (`KismetArrayLibrary.Array_Set` _array 0 (`|GetArrayItem` _array 1)))
    (`KismetArrayLibrary.Array_Set` _array 1)
    (else
      ;[1 1 1] N'as pas deja de couleur
      (`KismetArrayLibrary.Array_Add` _tp_all _nameref))))