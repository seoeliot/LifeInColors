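; Paintable physics cube, movable by conveyor belts, that respawns at its starting location and scale five seconds after being destroyed, including by falling too low.
; Color sets materials in the construction script and drives physics through OnChangeColor, which resets defaults first.
; Blue freezes, Yellow bounces and launches the player, Green rises by tick offset.
; Red slides on hit via a swept Timeline lerp, unless the hitter is tagged CantPushRedCube.
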(event `self.ReceiveBeginPlay`
  (`|ExecutionSequence`
    (:`then_0`
      ;[1 1 1] Ajoute le tag pour se faire bouger par le tapis roulant
      (bind _output_get (set `self.Tags` (`self.Tags`)))
      (bind _asgi_main (cast `/Game/MyGame/Data/GameInstance/GI_Main` (`GameplayStatics.GetGameInstance`)))
      (`KismetArrayLibrary.Array_AddUnique` _output_get (`/Game/MyGame/Data/GameInstance/GI_Main.TagNameTapisRoulant` _asgi_main)))
    (:`then_1`
      (`self.EventChangeColor`)
      (add `self.OnChangeColor` (`|CreateDelegate` :!event `EventChangeColor`))
      (set `self.startPosition` (`self.K2_GetActorLocation`))
      (set `self.startScale` (`self.GetActorScale3D`))
      (add `self.OnDestroyed` (delegate `OnDestroyed_Event_0`)))
    (:`then_2`
      (`KismetSystemLibrary.Delay` 2.0))))

(event `OnDestroyed_Event_0` :!signature `self.OnDestroyed`
  (params (DestroyedActor :type "Actor Object Reference"))
  (`KismetSystemLibrary.Delay` 5.0)
  (`|SpawnActorFromClass` "BP_PaintableCube5SecRespawn_C" (`KismetMathLibrary.MakeTransform` (`self.startPosition`) (struct) (`self.startScale`)) "Undefined" "OverrideRootScale" null null))

(event `EventChangeColor`
  (`self.ResetColor`)
  (switch `/Game/MyGame/Data/Enum_Struct/EnumColor` (`self.Color`)
    (:`NewEnumerator0`
      (`PrimitiveComponent.SetSimulatePhysics` (`self.StaticMesh`) false))
    (:`NewEnumerator2`
      (`self.SetPhysicsMaterial` "/Game/MyGame/Mech_Color/Paintable/Cube/BouncyCrate.BouncyCrate"))
    (:`NewEnumerator3`
      (`PrimitiveComponent.SetEnableGravity` (`self.StaticMesh`) false)
      (bind _asbp_first_person (cast `/Game/MyGame/Joueur/Character/BP_FirstPerson` (`GameplayStatics.GetPlayerPawn` 0)))
      (`KismetSystemLibrary.PrintString` "Hello")
      (if (`PrimitiveComponent.IsOverlappingActor` (`self.StaticMesh`) _asbp_first_person)
        (`PrimitiveComponent.SetSimulatePhysics` (`self.StaticMesh`) false)))))

(event `self.ReceiveTick`
  (params (DeltaSeconds :type "Float (single-precision)"))
  (bind (_returnvalue_x _returnvalue_y _returnvalue_z) (`KismetMathLibrary.BreakVector` (`self.K2_GetActorLocation`)))
  (`|ExecutionSequence`
    (:`then_0`
      (switch `/Game/MyGame/Data/Enum_Struct/EnumColor` (`self.Color`)
        (:`NewEnumerator3`
          (`SceneComponent.K2_AddWorldOffset` (`self.StaticMesh`) (* DeltaSeconds (0.0 0.0 200.0)) false false))))
    (:`then_1`
      (if (< _returnvalue_z -15000.0)
        (`self.K2_DestroyActor`)))))

(event `self.ReceiveHit`
  (params (MyComp :type "PrimitiveComponent Object Reference") (Other :type "Actor Object Reference") (OtherComp :type "PrimitiveComponent Object Reference") (bSelfMoved :type Boolean) (HitLocation :type "Vector Structure") (HitNormal :type "Vector Structure") (NormalImpulse :type "Vector Structure") (Hit :type "HitResult Structure (by ref)"))
  (switch `/Game/MyGame/Data/Enum_Struct/EnumColor` (`self.Color`)
    (:`NewEnumerator1`
      (if (not (`self.ActorHasTag` Other "CantPushRedCube"))
        ;[1 1 1] Comment
        (bind _newparam (`self.NewFunction_0` null HitNormal))
        (bind _output_get (set `self.redPushStartLocation` (`SceneComponent.K2_GetComponentLocation` (`self.StaticMesh`))))
        (bind (_returnvalue_x _returnvalue_y) (`KismetMathLibrary.BreakVector` (* _newparam (`self.redPushForce`))))
        (set `self.RedPushEndLocation` (+ _output_get (`KismetMathLibrary.MakeVector` _returnvalue_x _returnvalue_y 2.0)))
        (bind (_direction _newtrack_0) (`Timeline|Timeline_0` :!via `PlayFromStart`)
          (:`Update`
            (`SceneComponent.K2_SetWorldLocation` (`self.StaticMesh`) (`KismetMathLibrary.VLerp` (`self.redPushStartLocation`) (`self.RedPushEndLocation`) _newtrack_0) true true)
            (`KismetSystemLibrary.DrawDebugSphere` (`self.RedPushEndLocation`))))))
    (:`NewEnumerator2`
      (bind _asbp_first_person (cast `/Game/MyGame/Joueur/Character/BP_FirstPerson` Other))
      (bind (_returnvalue_x_2 _returnvalue_y_2 _returnvalue_z) (`KismetMathLibrary.BreakVector` (`SceneComponent.GetComponentVelocity` (`Actor.RootComponent` _asbp_first_person))))
      (`Character.LaunchCharacter` _asbp_first_person (`KismetMathLibrary.MakeVector` 0.0 0.0 (* (`KismetMathLibrary.FClamp` _returnvalue_z -4200.0 -420.0) -1.0)) false true))
    (:`NewEnumerator3`
      (`PrimitiveComponent.SetSimulatePhysics` (`self.StaticMesh`) false))))

(event `self.ReceiveActorEndOverlap`
  (params (OtherActor :type "Actor Object Reference"))
  (switch `/Game/MyGame/Data/Enum_Struct/EnumColor` (`self.Color`)
    (:`NewEnumerator3`
      (`PrimitiveComponent.SetSimulatePhysics` (`self.StaticMesh`) true))))

(fn `ChangeColor`
  (params (newColor :type "/Game/MyGame/Data/Enum_Struct/EnumColor Enum" :default "NewEnumerator0"))
  (bind (_mat_none _mat_blue _mat_green _mat_yellow _mat_red) (break `/Game/MyGame/Data/Enum_Struct/StructColorText` (`self.ColorTextures`)))
  (set `self.Color` newColor)
  (for (_array_element _array_index) (select `/Game/MyGame/Data/Enum_Struct/EnumColor` (`self.Color`) :`NewEnumerator0` _mat_blue :`NewEnumerator1` _mat_red :`NewEnumerator2` _mat_yellow :`NewEnumerator3` _mat_green :`NewEnumerator4` _mat_none)
    (`PrimitiveComponent.SetMaterial` (`self.StaticMesh`) _array_index _array_element)
    (`self.OnChangeColor`)))

(fn `NewFunction_0`
  (params (other :type "Actor Object Reference") (`Hit Impulse` :type "Vector Structure"))
  (returns (NewParam :type "Vector Structure"))
  (locals (NewLocalVar_0 :type "Vector Structure"))
  (bind _ascharacter (cast `Character` other)
    (:`then`
      (set `local.NewLocalVar_0` (`self.GetActorForwardVector` _ascharacter)))
    (:`CastFailed`
      (set `local.NewLocalVar_0` (`KismetMathLibrary.Normal` `Hit Impulse`))))
  (return (`local.NewLocalVar_0`)))

(fn `ResetColor`
  (bind _staticmesh (`self.StaticMesh`))
  (`self.SetPhysicsMaterial` "/Game/MyGame/Mech_Color/Paintable/Cube/DefaultPhysic.DefaultPhysic")
  (`PrimitiveComponent.SetSimulatePhysics` _staticmesh true)
  (`PrimitiveComponent.SetEnableGravity` _staticmesh true)
  (set `PrimitiveComponent.CanCharacterStepUpOn` "ECB_Yes" _staticmesh)
  (`PrimitiveComponent.AddImpulse` (`self.StaticMesh`) (0.0 0.0 1.0) "None" true))

(fn `SetPhysicsMaterial`
  (params (`new Physical Material` :type "PhysicalMaterial Object Reference"))
  (`PrimitiveComponent.SetPhysMaterialOverride` (`self.StaticMesh`) `new Physical Material`))

(fn `UserConstructionScript`
  (`self.ChangeColor` (`self.Color`)))