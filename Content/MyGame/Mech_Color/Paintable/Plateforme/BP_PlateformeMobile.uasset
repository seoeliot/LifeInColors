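; Paintable mobile platform whose color sets its behavior: Red moves, Blue halts with optional 90-degree rotation, Yellow halts and bounces characters along an arrow.
; A timeline lerps the mesh between two points with optional ping-pong, gated by a trigger-count energy check.
; Color changes swap material, play a paint sound and re-evaluate movement; stopping reverses instead when ForMehdi is set.
; An attached child actor follows every tick, and Yellow flags overlapping turret bullets.
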(event `/Game/MyGame/Mech_Color/Paintable/BPI_Paintable.ChangeColor`
  (params (newColor :type "/Game/MyGame/Data/Enum_Struct/EnumColor Enum" :default "NewEnumerator0"))
  (`self.UpdateMaterial` newColor)
  (`GameplayStatics.PlaySoundAtLocation` (select `/Game/MyGame/Data/Enum_Struct/EnumColor` (`self.EnumColor`) :`NewEnumerator0` "/Game/MyGame/Joueur/Gun/Sound/PaintSound/SFX_PaintBlue.SFX_PaintBlue" :`NewEnumerator1` "/Game/MyGame/Joueur/Gun/Sound/PaintSound/SFX_RedPaint.SFX_RedPaint" :`NewEnumerator2` "/Game/MyGame/Joueur/Gun/Sound/PaintSound/SFX_PaintYellow.SFX_PaintYellow" :!type "SoundBase Object Reference") (`self.K2_GetActorLocation`) (struct) 1.0 1.0 0.0 null null null null))

(event `self.ReceiveBeginPlay`
  (`|ExecutionSequence`
    (:`then_0`
      (`self.SetFiredOnEvent`))
    (:`then_1`
      (set `self.CustomTimeDilation` (`self.speed`))
      (`self.BeginFunction`)
      (set `self.BeginLoc` (+ (`self.K2_GetActorLocation`) (`self.BeginLoc`)))
      (set `self.EndLoc` (+ (`self.EndLoc`) (`self.K2_GetActorLocation`)))
      (`TimelineComponent.SetNewTime` (`self.Timeline_0`) (`self.Newtime`))
      (add `self.NewEventDispatcher_0` (delegate `EventOnChangeColor`))
      (add `self.StartPlatform` (delegate `EventStartPlatform`))
      (`self.CheckEnergy`
        (:`enoughEnergy`
          (`self.EventStartPlatform`)
          (`self.EventOnChangeColor`))))))

(event `EventStartPlatform`
  (switch `ETimelineDirection` (stale _direction)
    (:`Forward`
      (bind (_direction _newtrack_0) (`Timeline|Timeline_0` :!label _label)
        (:`Update`
          (`SceneComponent.K2_SetWorldLocation` (`self.PlateformeMesh`) (`KismetMathLibrary.VLerp` (`self.BeginLoc`) (`self.EndLoc`) _newtrack_0) false false))
        (:`Finished`
          (switch `ETimelineDirection` _direction
            (:`Forward`
              (if (`self.bPingPong`)
                (goto _label :!via `Reverse`)))
            (:`Backward`
              (`self.CheckEnergy`
                (:`enoughEnergy`
                  (goto _label))))))))
    (:`Backward`
      (goto _label :!via `Reverse`))))

(event `EventStopPlatform`
  (if (not (`self.ForMehdi`))
    (goto _label :!via `Stop`)
    (else
      (goto _label :!via `Reverse`))))

(event `EventOnChangeColor`
  (`self.CheckEnergy`
    (:`enoughEnergy`
      (`self.StartPlatform`))
    (:`notEnoughEnergy`
      (`self.EventStopPlatform`)))
  (set `self.CustomTimeDilation` (`self.speed`))
  (`self.K2_SetActorRotation` (struct))
  (switch `/Game/MyGame/Data/Enum_Struct/EnumColor` (`self.EnumColor`)
    (:`NewEnumerator0`
      (`|ExecutionSequence`
        (:`then_0`
          (if (`self.Rota 90y`)
            (`self.K2_SetActorRotation` (struct :`Pitch` 90.0))
            (elif (`self.Rota -90x`)
              (`self.K2_SetActorRotation` (struct :`Roll` -90.0))
              (elif (`self.Rota -90y`)
                (`self.K2_SetActorRotation` (struct :`Pitch` -90.0))
                (elif (`self.Rota 90x`)
                  (`self.K2_SetActorRotation` (struct :`Roll` 90.0)))))))
        (:`then_1`
          (`self.EventStopPlatform` :!label _label_2))))
    (:`NewEnumerator2`
      (goto _label_2))
    (:`NewEnumerator4`
      (goto _label_2))))

(event `self.ReceiveTick`
  (params (DeltaSeconds :type "Float (single-precision)"))
  (`self.SetChildActorPosition`))

(event `self.Action`
  (params (currentTrigger :type Integer))
  (`self.CheckEnergy`
    (:`enoughEnergy`
      (if (not (`self.ForMehdi`))
        (`self.EventStartPlatform`)
        (else
          (`self.EventStopPlatform` :!label _label_3))))
    (:`notEnoughEnergy`
      (goto _label_3))))

(event `self.PlateformeMesh.OnComponentHit`
  (params (HitComponent :type "PrimitiveComponent Object Reference") (OtherActor :type "Actor Object Reference") (OtherComp :type "PrimitiveComponent Object Reference") (NormalImpulse :type "Vector Structure") (Hit :type "HitResult Structure (by ref)"))
  (if (`|EnumEquality` (`self.EnumColor`) "NewEnumerator2")
    (bind _ascharacter (cast `Character` OtherActor))
    (`Character.LaunchCharacter` _ascharacter (* (`KismetMathLibrary.Abs` (`KismetMathLibrary.Vector_Distance` (0.0 0.0 0.0) (`SceneComponent.GetComponentVelocity` (`Actor.RootComponent` _ascharacter)))) (`KismetMathLibrary.Normal` (`SceneComponent.GetForwardVector` (`self.Arrow1`)))) false true)))

(event `self.BumpStart.OnComponentBeginOverlap`
  (params (OverlappedComponent :type "PrimitiveComponent Object Reference") (OtherActor :type "Actor Object Reference") (OtherComp :type "PrimitiveComponent Object Reference") (OtherBodyIndex :type Integer) (bFromSweep :type Boolean) (SweepResult :type "HitResult Structure (by ref)"))
  (if (`|EnumEquality` (`self.EnumColor`) "NewEnumerator2")
    (bind _asbp_turret_bullet (cast `/Game/MyGame/Mech_Color/Paintable/Tourelle/BP_TurretBullet` OtherActor))
    (set `/Game/MyGame/Mech_Color/Paintable/Tourelle/BP_TurretBullet.TouchBumpActor` true _asbp_turret_bullet)))

(event `self.BumpStart.OnComponentEndOverlap`
  (params (OverlappedComponent :type "PrimitiveComponent Object Reference") (OtherActor :type "Actor Object Reference") (OtherComp :type "PrimitiveComponent Object Reference") (OtherBodyIndex :type Integer))
  (bind _asbp_turret_bullet (cast `/Game/MyGame/Mech_Color/Paintable/Tourelle/BP_TurretBullet` OtherActor))
  (set `/Game/MyGame/Mech_Color/Paintable/Tourelle/BP_TurretBullet.TouchBumpActor` false _asbp_turret_bullet))

(fn `ResetColor`)

(fn `SetChildActorPosition`
  (bind _childactorpivot (`self.ChildActorPivot`))
  (bind _childactor (`self.childActor`))
  (bind (_childactorrotation_x _childactorrotation_y _childactorrotation_z) (`KismetMathLibrary.BreakVector` (`self.childActorRotation`)))
  (`/Engine/EditorBlueprintResources/StandardMacros.IsValid` _childactor
    (:`Is Valid`
      (bind _asbp_color_detector (cast `/Game/MyGame/Mech_Env/ColorDetector/BP_ColorDetector` _childactor)
        (:`then`
          (set `/Game/MyGame/Mech_Env/ColorDetector/BP_ColorDetector.parentPlatform` self _asbp_color_detector))
        (:`CastFailed`
          _))
      (`self.K2_SetActorLocation` (`self.childActor`) (+ (`SceneComponent.K2_GetComponentLocation` (`self.PlateformeMesh`)) (`self.childActorOffset`)) false false)
      (`SceneComponent.K2_SetRelativeRotation` _childactorpivot (`KismetMathLibrary.MakeRotator` _childactorrotation_x _childactorrotation_y _childactorrotation_z) false false)
      (`self.K2_SetActorRotation` (`self.childActor`) (`SceneComponent.K2_GetComponentRotation` _childactorpivot) false))))

(fn `SetFiredOnEvent`)

(fn `UpdateMaterial`
  (params (newColor :type "/Game/MyGame/Data/Enum_Struct/EnumColor Enum" :default "NewEnumerator0"))
  (set `self.EnumColor` newColor)
  (`PrimitiveComponent.SetMaterial` (`self.PlateformeMesh`) 0 (`|GetArrayItem` (`self.ColorMaterials`) (select `/Game/MyGame/Data/Enum_Struct/EnumColor` (`self.EnumColor`) :`NewEnumerator0` 2 :`NewEnumerator1` 1 :`NewEnumerator2` 3)))
  (`self.NewEventDispatcher_0`))

(fn `UserConstructionScript`
  (`self.ConstructionFunction`)
  (`PrimitiveComponent.SetMaterial` (`self.PlateformeMesh`) 0 (`|GetArrayItem` (`self.ColorMaterials`) (select `/Game/MyGame/Data/Enum_Struct/EnumColor` (`self.EnumColor`) :`NewEnumerator0` 2 :`NewEnumerator1` 1 :`NewEnumerator2` 3)))
  (`SceneComponent.SetWorldScale3D` (`self.Arrow1`) (1.0 1.0 1.0))
  (`self.SetChildActorPosition`))