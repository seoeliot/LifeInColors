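; BP_Paintable is a paintable object for the color mechanic, whose static mesh changes materials to match its paint color.
; SetColor, gated by CanChangeColor, stores the new PaintColor and picks that color's material array from PaintColorMaterials, including a None set.
; It applies the array to the mesh by slot index, calling the empty OnChangeColor hook after each slot rather than once per change.
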(fn `OnChangeColor`)

(fn `SetColor`
  (params (NewColor :type "/Game/MyGame/Data/Enum_Struct/EnumColor Enum" :default "NewEnumerator0"))
  (locals (NewLocalVar_0 :type "Array of Material Object Reference"))
  (bind (_mat_none _mat_blue _mat_green _mat_yellow _mat_red) (break `/Game/MyGame/Data/Enum_Struct/StructColorText` (`self.PaintColorMaterials`)))
  (if (`self.CanChangeColor`)
    (bind _output_get (set `self.PaintColor` NewColor))
    (switch `/Game/MyGame/Data/Enum_Struct/EnumColor` _output_get
      (:`NewEnumerator0`
        (set `local.NewLocalVar_0` _mat_blue))
      (:`NewEnumerator1`
        (set `local.NewLocalVar_0` _mat_red))
      (:`NewEnumerator2`
        (set `local.NewLocalVar_0` _mat_yellow))
      (:`NewEnumerator3`
        (set `local.NewLocalVar_0` _mat_green))
      (:`NewEnumerator4`
        (set `local.NewLocalVar_0` _mat_none)))
    (for (_array_element _array_index) (`local.NewLocalVar_0`)
      (`PrimitiveComponent.SetMaterial` (`self.StaticMesh`) _array_index _array_element)
      (`self.OnChangeColor`))))

(fn `UserConstructionScript`)